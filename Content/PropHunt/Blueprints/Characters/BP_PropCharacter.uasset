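; Player character for the prop team in Prop Hunt, disguising itself as a world prop.
; A camera trace picks a BP_BaseProp whose mesh the server copies while hiding the body, with a random auto-hide at play time start.
; Point damage feeds the health manager, shows a damage indicator, and on death notifies the game mode and ragdolls the body.
; Also handles movement, a camera-orbit lock, and random sounds with cooldown, using RepNotifies for visibility and audio.
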(event `InputAction|Hide`
  (params (Key :type "Key Structure"))
  (bind (_start _end) (`self.F_GetDefaultTrace` 700.0))
  ;[0 1 0.7371] Hide
  (:`Pressed`
    (bind (_outhit _returnvalue) (`KismetSystemLibrary.LineTraceSingle` _start _end "TraceTypeQuery1"))
    (if _returnvalue
      (bind _asbp_base_prop (cast `/Game/PropHunt/Blueprints/Props/BP_BaseProp` (`.HitActor` (`GameplayStatics.BreakHitResult` _outhit))))
      (`self.SRV_Hide` _asbp_base_prop))))

(event `self.ReceiveBeginPlay`
  ;[1 1 1] Begin play. Autohide at play time start if player is not hidden
  (add `/Game/PropHunt/Blueprints/Kernel/BP_Kernel_GS.D_PlayTime` (`/Game/PropHunt/Blueprints/Helpers/BP_Helpers.H_KernelGS`) (delegate `E_AutoHide`)))

(event `E_AutoHide`
  ;[1 1 1] Begin play. Autohide at play time start if player is not hidden
  (`/Engine/EditorBlueprintResources/StandardMacros.IsValid` (`StaticMeshComponent.StaticMesh` (`self.PropMesh`))
    (:`Is Not Valid`
      (bind _outactors (`GameplayStatics.GetAllActorsOfClass` "/Game/PropHunt/Blueprints/Props/BP_BaseProp.BP_BaseProp_C"))
      (bind _output (`|GetArrayItem` _outactors (`KismetMathLibrary.RandomInteger` (`KismetArrayLibrary.Array_Length` _outactors))))
      (`/Engine/EditorBlueprintResources/StandardMacros.IsValid` _output
        (:`Is Valid`
          (`self.SRV_Hide` _output))))))

(event `SRV_Hide`
  (params (Prop :type "/Game/PropHunt/Blueprints/Props/BP_BaseProp Object Reference"))
  ;[0 1 0.7371] Hide
  (`StaticMeshComponent.SetStaticMesh` (`self.PropMesh`) (`StaticMeshComponent.StaticMesh` (`/Game/PropHunt/Blueprints/Props/BP_BaseProp.PropSM` Prop)))
  (set `self.IsVisible` false))

(event `/Game/PropHunt/Blueprints/Interfaces/BP_I_BaseCharacter.IE_DestroySelf`
  ;[1 1 1] Destroy character
  (`self.K2_DestroyActor`))

(event `InputAxis|MoveForward` :overrideparent false
  (params (AxisValue :type "Float (single-precision)"))
  ;[0 0.978 1] Movement input - WASD
  (bind _output_get (set `self.MoveForwardAxisValue` AxisValue))
  (`self.AddMovementInput` (`KismetMathLibrary.GetForwardVector` (`KismetMathLibrary.MakeRotator` 0.0 0.0 (.yaw (`self.GetControlRotation`)))) _output_get)
  (bind (_moveforward _moveright) (`self.F_CalculateMovement`))
  (`self.SRV_UpdateDirection` _moveforward _moveright (`self.MoveRightAxisValue`)))

(event `CL_ShowDamageIndicator`
  (params (BulletTraceStart :type "Vector Structure"))
  ;[0.6172 0 1] Show damage indicator on client
  (bind _returnvalue (`|CreateWidget` "/Game/PropHunt/Blueprints/Widgets/Game/BP_W_DamageIndicator.BP_W_DamageIndicator_C" (`GameplayStatics.GetPlayerController` 0) BulletTraceStart))
  (`UserWidget.AddToViewport` _returnvalue 0))

(event `InputAxis|MoveRight` :overrideparent false
  (params (AxisValue :type "Float (single-precision)"))
  ;[0 0.978 1] Movement input - WASD
  (bind _output_get (set `self.MoveRightAxisValue` AxisValue))
  (`self.AddMovementInput` (`KismetMathLibrary.GetRightVector` (`KismetMathLibrary.MakeRotator` 0.0 0.0 (.yaw (`self.GetControlRotation`)))) _output_get))

(event `SRV_UpdateDirection`
  (params (MoveForward :type "Float (double-precision)") (MoveRight :type "Float (double-precision)") (MoveRightAxisValue :type "Float (double-precision)"))
  ;[0 0.978 1] Movement input - WASD
  (set `self.MoveForward` MoveForward)
  (set `self.MoveRight` MoveRight)
  (set `self.MoveRightAxisValue` MoveRightAxisValue))

(event `self.ReceivePointDamage`
  (params (Damage :type "Float (single-precision)") (DamageType :type "DamageType Object Reference") (HitLocation :type "Vector Structure") (HitNormal :type "Vector Structure") (HitComponent :type "PrimitiveComponent Object Reference") (BoneName :type Name) (ShotFromDirection :type "Vector Structure") (InstigatedBy :type "Controller Object Reference") (DamageCauser :type "Actor Object Reference") (HitInfo :type "HitResult Structure (by ref)"))
  ;[0.6144 0 1] Point damage
  (if (not (`self.IsDead`))
    (`self.CL_ShowDamageIndicator` (`.TraceStart` (`GameplayStatics.BreakHitResult` HitInfo)))
    (bind _isdead (`/Game/PropHunt/Blueprints/Characters/BP_HealthManager.FS_ApplyDamage` (`self.BP_HealthManager`) Damage))
    (if _isdead
      (set `self.IsDead` true)
      (`/Game/PropHunt/Blueprints/Kernel/BP_Kernel_GM.FS_ProcessPlayerDeath` (`/Game/PropHunt/Blueprints/Helpers/BP_Helpers.H_KernelGM`) (`self.PlayerState`) (`Controller.PlayerState` InstigatedBy) (`/Game/PropHunt/Blueprints/Weapons/BP_FirearmWeapon.WeaponId` (cast `/Game/PropHunt/Blueprints/Weapons/BP_FirearmWeapon` DamageCauser :!pure true)))
      (`self.MC_Death`)
      (`self.SetLifeSpan` 5.0))))

(event `InputAction|Jump` :overrideparent false
  (params (Key :type "Key Structure"))
  ;[0.9361 0.1939 1] SPACE - Jump
  (:`Pressed`
    (`self.Jump`))
  (:`Released`
    (`self.StopJumping`)))

(event `InputAxis|Turn` :overrideparent false
  (params (AxisValue :type "Float (single-precision)"))
  ;[0 1 0.9414] mouse - Turn
  (if (`self.Locked`)
    (`SceneComponent.K2_AddLocalRotation` (`self.SpringArm`) (`KismetMathLibrary.MakeRotator` 0.0 0.0 AxisValue) false false)
    (else
      (`self.AddControllerYawInput` AxisValue))))

(event `InputAxis|LookUp` :overrideparent false
  (params (AxisValue :type "Float (single-precision)"))
  ;[0 1 0.9414] mouse - Look up
  (if (not (`self.Locked`))
    (`self.AddControllerPitchInput` AxisValue)))

(event `MC_Death`
  ;[0.6172 0 1] Multicast death
  (`ActorComponent.K2_DestroyComponent` (`self.PropMesh`))
  (`SceneComponent.SetVisibility` (`self.Mesh`) true false)
  (`PrimitiveComponent.SetSimulatePhysics` (`self.Mesh`) true)
  (`PrimitiveComponent.SetCollisionEnabled` (`self.CapsuleComponent`) "NoCollision"))

(event `Key|F`
  (params (Key :type "Key Structure"))
  ;[1 1 1] Play Sound
  (:`Pressed`
    (if (`self.SoundOnDelay`)
      (`KismetSystemLibrary.PrintString` "Sound on cooldown! Chill bro")
      (else
        (`self.PlaySoundServer`)))))

(event `PlaySoundServer`
  (bind _soundwave (`self.SoundWave`))
  ;[1 1 1] Play Sound
  (set `self.PlaySound` (`|GetArrayItem` _soundwave (`KismetMathLibrary.RandomInteger` (`KismetArrayLibrary.Array_Length` _soundwave))))
  (`self.PlaySoundMulti`))

(event `PlaySoundMulti`
  ;[1 1 1] Play Sound
  (set `self.Pressed` true)
  (set `self.SoundOnDelay` true)
  (`KismetSystemLibrary.Delay` 5.0)
  (set `self.SoundOnDelay` false)
  (`KismetSystemLibrary.PrintString` "Sound ready" true false (struct :`R` 1.0 :`G` 0.080674 :`B` 0.385157 :`A` 0.64) 1.0))

(event `Key|G`
  (params (Key :type "Key Structure"))
  (bind _springarm (`self.SpringArm`))
  ;[1 1 1] Lock
  (:`Pressed`
    (`/Engine/EditorBlueprintResources/StandardMacros.FlipFlop`
      (:`A`
        (set `self.Locked` true)
        (set `SpringArmComponent.bUsePawnControlRotation` false _springarm))
      (:`B`
        (set `self.Locked` false)
        (set `SpringArmComponent.bUsePawnControlRotation` true _springarm)
        (`SceneComponent.K2_AddLocalRotation` :`self` _springarm)))))

(fn `F_CalculateMovement`
  (returns (MoveForward :type "Float (double-precision)") (MoveRight :type "Float (double-precision)"))
  (bind _moveforwardaxisvalue (`self.MoveForwardAxisValue`))
  (bind _moverightaxisvalue (`self.MoveRightAxisValue`))
  (bind _yaw (.yaw (`KismetMathLibrary.NormalizedDeltaRotator` (`self.GetControlRotation`) (`self.K2_GetActorRotation`))))
  (bind _returnvalue (- 0.0 _yaw))
  (`|ExecutionSequence`
    (:`then_0`
      (bind _output_get (set `self.MoveForward` (+ (* _moveforwardaxisvalue (`KismetMathLibrary.DegCos` _yaw)) (* (`KismetMathLibrary.DegSin` _returnvalue) _moverightaxisvalue)))))
    (:`then_1`
      (bind _output_get_2 (set `self.MoveRight` (+ (* _moveforwardaxisvalue (`KismetMathLibrary.DegSin` _yaw)) (* (`KismetMathLibrary.DegCos` _returnvalue) _moverightaxisvalue))))
      (return _output_get _output_get_2))))

(fn `F_GetDefaultTrace`
  (params (Lenght :type "Float (double-precision)"))
  (returns (Start :type "Vector Structure") (End :type "Vector Structure"))
  (bind _followcamera (`self.FollowCamera`))
  (bind _returnvalue (`SceneComponent.K2_GetComponentLocation` _followcamera))
  (bind _returnvalue_2 (`SceneComponent.GetForwardVector` _followcamera))
  (return (+ _returnvalue (* _returnvalue_2 300.0)) (+ _returnvalue (* _returnvalue_2 Lenght))))

(fn `IF_GetFollowCamera`
  (returns (Camera :type "CameraComponent Object Reference"))
  (return (`self.FollowCamera`)))

(fn `IF_GetHealth`
  (returns (Health :type "Float (double-precision)"))
  (return (`/Game/PropHunt/Blueprints/Characters/BP_HealthManager.Health` (`self.BP_HealthManager`))))

(fn `IF_GetTeam`
  (returns (Team :type Integer))
  (bind _team (message `/Game/PropHunt/Blueprints/Interfaces/BP_I_TeamPlayer.IF_GetTeam` (`self.PlayerState`)))
  (return _team))

(fn `IF_IsDead`
  (returns (IsDead :type Boolean))
  (return (`self.IsDead`)))

(fn `IF_SetHealth`
  (params (NewHealth :type "Float (double-precision)"))
  (returns (Health :type "Float (double-precision)"))
  (bind _output_get (set `/Game/PropHunt/Blueprints/Characters/BP_HealthManager.Health` NewHealth (`self.BP_HealthManager`)))
  (return _output_get))

(fn `IF_SetTeam`
  (params (NewTeam :type Integer))
  (returns (Team :type Integer))
  (bind _team (message `/Game/PropHunt/Blueprints/Interfaces/BP_I_TeamPlayer.IF_SetTeam` (`self.PlayerState`) NewTeam))
  (return _team))

(fn `OnRep_IsDead`
  (`/Engine/EditorBlueprintResources/ActorMacros.Switch Has Authority`
    (:`Authority`
      (bind _asbp_kernel_ps (cast `/Game/PropHunt/Blueprints/Kernel/BP_Kernel_PS` (`self.PlayerState`)))
      (set `/Game/PropHunt/Blueprints/Kernel/BP_Kernel_PS.IsDead` true _asbp_kernel_ps))))

(fn `OnRep_IsVisible`
  (`SceneComponent.SetVisibility` (`self.Mesh`) false false))

(fn `OnRep_PlaySound`)

(fn `OnRep_Pressed`
  (`GameplayStatics.SpawnSoundAttached` (`self.PlaySound`) (`self.CapsuleComponent`) "None" (0.0 0.0 0.0) (struct) "KeepRelativeOffset" false 0.7 1.0 0.0 "/Game/PropHunt/Sounds/SoundAttenuation.SoundAttenuation" null))

(fn `UserConstructionScript`)