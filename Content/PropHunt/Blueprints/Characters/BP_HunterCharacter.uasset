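; Player character for hunters in Prop Hunt, with input disabled while props hide at round start.
; Movement, sprint, crouch and aim set walk speed locally and mirror state through SRV events.
; Weapon input routes to BPWeaponsManager, while interface functions expose health, ammo, team and camera.
; Shooting a non-player prop damages the hunter through BPHealthManager; death is reported to the game mode, then multicasts a ragdoll and destroys weapons.
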(event `CL_ShowDamageIndicator`
  ;[0.1302 1 0.03963] Show damage indicator on client. It's auto removed from parent after 0.5 seconds
  (bind _returnvalue (`|CreateWidget` "/Game/PropHunt/Blueprints/Widgets/Game/BP_W_HunterDamageIndicator.BP_W_HunterDamageIndicator_C" (`GameplayStatics.GetPlayerController` 0)))
  (`UserWidget.AddToViewport` _returnvalue 22))

(event `self.ReceiveBeginPlay`
  ;[1 0.5268 0] BEGIN PLAY
  (`|ExecutionSequence`
    (:`then_0`
      ;;[1 1 1] disable input when props are hiding
      (`self.CL_DisableInput` (`KismetMathLibrary.Conv_IntToDouble` (`/Game/PropHunt/Blueprints/Kernel/BP_Kernel_GS.RoundStartTimeS` (`/Game/PropHunt/Blueprints/Helpers/BP_Helpers.H_KernelGS`)))))
    (:`then_1`
      ;;[1 1 1] Enable input on play time start
      (add `/Game/PropHunt/Blueprints/Kernel/BP_Kernel_GS.D_PlayTime` (`/Game/PropHunt/Blueprints/Helpers/BP_Helpers.H_KernelGS`) (delegate `E_EnableInputAtPlayTimeStart`)))))

(event `SRV_ApplyDamage`
  (bind _playerstate (`self.PlayerState`))
  ;[1 0 0.2295] Apply damage if hunter shots it prop which is not hidden player
  (bind _isdead (`/Game/PropHunt/Blueprints/Characters/BP_HealthManager.FS_ApplyDamage` (`self.BP_HealthManager`) (`self.WrongPropDamage`)))
  (`self.CL_ShowDamageIndicator`)
  (if _isdead
    (set `self.IsDead` true)
    (`/Game/PropHunt/Blueprints/Kernel/BP_Kernel_GM.FS_ProcessPlayerDeath` (`/Game/PropHunt/Blueprints/Helpers/BP_Helpers.H_KernelGM`) _playerstate _playerstate 2)
    (`self.MC_Death`)
    (`self.SetLifeSpan` 5.0)
    (`/Game/PropHunt/Blueprints/Characters/BP_WeaponsManager.FS_DestroyAllWeapons` (`self.BP_WeaponsManager`))))

(event `E_EnableInputAtPlayTimeStart`
  (bind _returnvalue (`self.GetController`))
  ;[1 0.5268 0] BEGIN PLAY
  ;;[1 1 1] Enable input on play time start
  (`/Engine/EditorBlueprintResources/StandardMacros.IsValid` _returnvalue
    (:`Is Valid`
      _)
    (:`Is Not Valid`
      (`KismetSystemLibrary.Delay` 1.0)))
  (`self.EnableInput` (cast `PlayerController` _returnvalue :!pure true)))

(event `/Game/PropHunt/Blueprints/Interfaces/BP_I_BaseCharacter.IE_DestroySelf`
  ;[1 0 0.05349] Destroy character and his weapons
  (`/Game/PropHunt/Blueprints/Characters/BP_WeaponsManager.FS_DestroyAllWeapons` (`self.BP_WeaponsManager`))
  (`self.K2_DestroyActor`))

(event `MC_Death`
  ;[1 0 0.01335] Multicast death
  (`PrimitiveComponent.SetSimulatePhysics` (`self.Mesh`) true)
  (`PrimitiveComponent.SetCollisionEnabled` (`self.CapsuleComponent`) "NoCollision")
  (`PrimitiveComponent.AddImpulseAtLocation` (`self.Mesh`) (0.0 0.0 10000.0) (`SceneComponent.GetSocketLocation` (`self.Mesh`) "head") "head"))

(event `/Game/PropHunt/Blueprints/Interfaces/BP_I_ArmedCharacter.IE_EquipWeapon`
  (params (Weapon :type "Actor Object Reference"))
  ;[1 0.6141 0.3474] Equip weapon
  (bind _asbp_firearm_weapon (cast `/Game/PropHunt/Blueprints/Weapons/BP_FirearmWeapon` Weapon))
  (`/Game/PropHunt/Blueprints/Weapons/BP_FirearmWeapon.EA_Equip` _asbp_firearm_weapon))

(event `CL_DisableInput`
  (params (Time :type "Float (double-precision)"))
  (bind _asplayer_controller (cast `PlayerController` (`self.GetController`) :!pure true))
  ;[1 1 1] Disable input
  (`self.DisableInput` _asplayer_controller)
  (`KismetSystemLibrary.Delay` Time)
  (`self.EnableInput` _asplayer_controller))

(event `/Game/PropHunt/Blueprints/Interfaces/BP_I_ArmedCharacter.IE_HolsterWeapon`
  (params (Weapon :type "Actor Object Reference"))
  ;[1 0.6141 0.3474] Equip weapon
  (bind _asbp_firearm_weapon (cast `/Game/PropHunt/Blueprints/Weapons/BP_FirearmWeapon` Weapon))
  (`/Game/PropHunt/Blueprints/Weapons/BP_FirearmWeapon.EA_Holster` _asbp_firearm_weapon))

(event `InputAction|EquipPrimaryWeapon`
  (params (Key :type "Key Structure"))
  ;[0.8438 0 0.02777] WEAPON CHANGE - 1,2, mouse up / down
  (:`Pressed`
    (`/Game/PropHunt/Blueprints/Characters/BP_WeaponsManager.E_EquipSelectedWeapon` (`self.BP_WeaponsManager`) 0)))

(event `InputAction|EquipSecondaryWeapon`
  (params (Key :type "Key Structure"))
  ;[0.8438 0 0.02777] WEAPON CHANGE - 1,2, mouse up / down
  (:`Pressed`
    (`/Game/PropHunt/Blueprints/Characters/BP_WeaponsManager.E_EquipSelectedWeapon` (`self.BP_WeaponsManager`) 1)))

(event `InputAxis|MoveForward` :overrideparent false
  (params (AxisValue :type "Float (single-precision)"))
  ;[0 0.978 1] Movement input - WASD
  (bind _output_get (set `self.MoveForwardAxisValue` AxisValue))
  (`self.AddMovementInput` (`KismetMathLibrary.GetForwardVector` (`KismetMathLibrary.MakeRotator` 0.0 0.0 (.yaw (`self.GetControlRotation`)))) _output_get)
  (bind (_moveforward _moveright) (`self.F_CalculateMovement`))
  (`self.SRV_UpdateDirection` _moveforward _moveright (`self.MoveRightAxisValue`)))

(event `InputAction|NextWeapon`
  (params (Key :type "Key Structure"))
  ;[0.8438 0 0.02777] WEAPON CHANGE - 1,2, mouse up / down
  (:`Pressed`
    (`/Game/PropHunt/Blueprints/Characters/BP_WeaponsManager.E_ScrollWeaponChange` (`self.BP_WeaponsManager`) :!label _label)))

(event `InputAction|LMB`
  (params (Key :type "Key Structure"))
  ;[0.8438 0 0.02777] LMB - Shoot pressed
  (:`Pressed`
    (set `self.IsShooting` true)
    (`self.F_StopSprint`)
    (`/Game/PropHunt/Blueprints/Characters/BP_WeaponsManager.E_ShootPressed` (`self.BP_WeaponsManager`)))
  (:`Released`
    (set `self.IsShooting` false)
    (`/Game/PropHunt/Blueprints/Characters/BP_WeaponsManager.E_ShootReleased` (`self.BP_WeaponsManager`))))

(event `InputAxis|Turn` :overrideparent false
  (params (AxisValue :type "Float (single-precision)"))
  ;[0 1 0.9414] mouse - Turn
  (`self.AddControllerYawInput` AxisValue))

(event `InputAction|PreviousWeapon`
  (params (Key :type "Key Structure"))
  ;[0.8438 0 0.02777] WEAPON CHANGE - 1,2, mouse up / down
  (:`Pressed`
    (goto _label)))

(event `InputAxis|MoveRight` :overrideparent false
  (params (AxisValue :type "Float (single-precision)"))
  ;[0 0.978 1] Movement input - WASD
  (bind _output_get (set `self.MoveRightAxisValue` AxisValue))
  (`self.AddMovementInput` (`KismetMathLibrary.GetRightVector` (`KismetMathLibrary.MakeRotator` 0.0 0.0 (.yaw (`self.GetControlRotation`)))) _output_get))

(event `InputAction|RMB`
  (params (Key :type "Key Structure"))
  (bind _equipedweapon (`/Game/PropHunt/Blueprints/Characters/BP_WeaponsManager.EquipedWeapon` (`self.BP_WeaponsManager`)))
  ;[0.8438 0 0.02777] RMB - AIM
  (:`Pressed`
    (`self.F_StopSprint`)
    (`self.SRV_Aim` true)
    (set `self.IsAiming` true)
    (`self.F_SetAimSpeed`)
    (bind _asbp_firearm_weapon (cast `/Game/PropHunt/Blueprints/Weapons/BP_FirearmWeapon` _equipedweapon :!label _label_2))
    (`/Engine/EditorBlueprintResources/StandardMacros.IsValid` _equipedweapon
      (:`Is Valid`
        (message `/Game/PropHunt/Blueprints/Interfaces/BP_I_Weapon.IE_Aim` _asbp_firearm_weapon (`self.IsAiming`)))))
  (:`Released`
    (`self.SRV_Aim` false)
    (set `self.IsAiming` false)
    (`self.F_SetAimSpeed`)
    (goto _label_2)))

(event `InputAction|Jump` :overrideparent false
  (params (Key :type "Key Structure"))
  ;[0.9361 0.1939 1] SPACE - Jump
  (:`Pressed`
    (`self.F_Jump`))
  (:`Released`
    (`self.StopJumping`)))

(event `InputAxis|LookUp` :overrideparent false
  (params (AxisValue :type "Float (single-precision)"))
  ;[0 1 0.9414] mouse - Look up
  (`self.AddControllerPitchInput` AxisValue))

(event `SRV_UpdateDirection`
  (params (MoveForward :type "Float (double-precision)") (MoveRight :type "Float (double-precision)") (MoveRightAxisValue :type "Float (double-precision)"))
  ;[0 0.978 1] Movement input - WASD
  (set `self.MoveForward` MoveForward)
  (set `self.MoveRight` MoveRight)
  (bind _output_get (set `self.MoveRightAxisValue` MoveRightAxisValue))
  (if (!= _output_get 0.0)
    (set `self.IsSprinting` false)))

(event `SRV_Aim`
  (params (IsAiming :type Boolean))
  ;[0.8438 0 0.02777] RMB - AIM
  (set `self.IsAiming` IsAiming)
  (`self.F_SetAimSpeed`))

(event `InputAction|Sprint`
  (params (Key :type "Key Structure"))
  ;[0.9361 0.1939 1] SHIFT - Sprint
  (:`Pressed`
    (if (`self.IsCrouching`)
      (set `self.IsCrouching` false)
      (`self.E_CameraCrouchEffect`))
    (if (not (`self.IsShooting`))
      (`self.F_Sprint`)))
  (:`Released`
    (`self.SRV_Sprint` false)
    (`self.F_SetSprintSpeed` false)))

(event `InputAction|Crouch`
  (params (Key :type "Key Structure"))
  ;[0.9361 0.1939 1] CTRL - Crouch
  (:`Pressed`
    (if (`self.IsCrouching`)
      (`self.SRV_Crouch` false)
      (set `self.IsCrouching` false)
      (else
        (`self.SRV_Crouch` true)
        (set `self.IsCrouching` true)))
    (`self.F_SetCrouchSpeed`)
    (`self.E_CameraCrouchEffect`)))

(event `InputAction|Reload`
  (params (Key :type "Key Structure"))
  ;[0.8438 0 0.02777] Reload
  (:`Pressed`
    (set `self.IsShooting` false)
    (`/Game/PropHunt/Blueprints/Interfaces/BP_I_ArmedCharacter.IE_Reload`)))

(event `SRV_Crouch`
  (params (IsCrouching :type Boolean))
  ;[0.9361 0.1939 1] CTRL - Crouch
  (set `self.IsCrouching` IsCrouching)
  (`self.F_SetCrouchSpeed`))

(event `SRV_Sprint`
  (params (IsSptinting :type Boolean))
  ;[0.9361 0.1939 1] SHIFT - Sprint
  (`self.FS_Sprint` IsSptinting))

(event `/Game/PropHunt/Blueprints/Interfaces/BP_I_ArmedCharacter.IE_Reload`
  ;[0.8438 0 0.02777] Reload
  (`/Game/PropHunt/Blueprints/Characters/BP_WeaponsManager.E_Reload` (`self.BP_WeaponsManager`)))

(event `E_CameraCrouchEffect`
  ;[1 1 1] Change camera location on crouch
  (if (`self.IsCrouching`)
    (bind (_direction _camerazlocation) (`Timeline|Timeline_0` :!via `ReverseFromEnd` :!label _label_3)
      (:`Update`
        (`SceneComponent.K2_SetRelativeLocation` (`self.FollowCamera`) (`KismetMathLibrary.MakeVector` 147.0 42.0 _camerazlocation) false false)))
    (else
      (goto _label_3 :!via `PlayFromStart`))))

(fn `F_CalculateMovement`
  (returns (MoveForward :type "Float (double-precision)") (MoveRight :type "Float (double-precision)"))
  (bind _moveforwardaxisvalue (`self.MoveForwardAxisValue`))
  (bind _moverightaxisvalue (`self.MoveRightAxisValue`))
  (bind _yaw (.yaw (`KismetMathLibrary.NormalizedDeltaRotator` (`self.GetControlRotation`) (`self.K2_GetActorRotation`))))
  (bind _returnvalue (- 0.0 _yaw))
  (`|ExecutionSequence`
    (:`then_0`
      (bind _output_get (set `self.MoveForward` (+ (* _moveforwardaxisvalue (`KismetMathLibrary.DegCos` _yaw)) (* (`KismetMathLibrary.DegSin` _returnvalue) _moverightaxisvalue)))))
    (:`then_1`
      (bind _output_get_2 (set `self.MoveRight` (+ (* _moveforwardaxisvalue (`KismetMathLibrary.DegSin` _yaw)) (* (`KismetMathLibrary.DegCos` _returnvalue) _moverightaxisvalue))))
      (return _output_get _output_get_2))))

(fn `F_GetDefaultTrace`
  (params (Lenght :type "Float (double-precision)"))
  (returns (Start :type "Vector Structure") (End :type "Vector Structure"))
  (bind _followcamera (`self.FollowCamera`))
  (bind _returnvalue (`SceneComponent.K2_GetComponentLocation` _followcamera))
  (bind _returnvalue_2 (`SceneComponent.GetForwardVector` _followcamera))
  (return (+ _returnvalue (* _returnvalue_2 300.0)) (+ _returnvalue (* _returnvalue_2 Lenght))))

(fn `F_Jump`
  (`|ExecutionSequence`
    (:`then_0`
      (if (`self.IsCrouching`)
        (set `self.IsCrouching` false)
        (`self.SRV_Crouch` false)
        (`self.E_CameraCrouchEffect`)
        (else
          (`self.Jump`))))
    (:`then_1`
      (if (`self.IsSprinting`)
        (`self.SRV_Sprint` false)
        (`self.Jump`)))))

(fn `F_SetAimSpeed`
  (bind _charactermovement (`self.CharacterMovement`))
  (if (`self.IsAiming`)
    (set `CharacterMovementComponent.MaxWalkSpeed` (`self.AimSpeed`) _charactermovement)
    (elif (`self.IsCrouching`)
      (set `CharacterMovementComponent.MaxWalkSpeed` (`self.CrouchSpeed`) _charactermovement)
      (else
        (set `CharacterMovementComponent.MaxWalkSpeed` (`self.JogSpeed`) _charactermovement)))))

(fn `F_SetCrouchSpeed`
  (bind _charactermovement (`self.CharacterMovement`))
  (if (`self.IsCrouching`)
    (set `CharacterMovementComponent.MaxWalkSpeed` (`self.CrouchSpeed`) _charactermovement)
    (else
      (set `CharacterMovementComponent.MaxWalkSpeed` (`self.JogSpeed`) _charactermovement))))

(fn `F_SetSprintSpeed`
  (params (Sprint :type Boolean))
  (bind _charactermovement (`self.CharacterMovement`))
  (if Sprint
    (set `CharacterMovementComponent.MaxWalkSpeed` (`self.SprintSpeed`) _charactermovement)
    (else
      (set `CharacterMovementComponent.MaxWalkSpeed` (`self.JogSpeed`) _charactermovement))))

(fn `F_Sprint`
  (set `self.IsAiming` false)
  (set `self.IsSprinting` true)
  (`self.SRV_Sprint` true)
  (`self.F_SetSprintSpeed` true))

(fn `F_StopSprint`
  (if (`self.IsSprinting`)
    (`self.F_SetSprintSpeed` false)
    (`self.SRV_Sprint` false)))

(fn `FS_Sprint`
  (params (IsSprinting :type Boolean))
  (`|ExecutionSequence`
    (:`then_0`
      (if (`self.IsCrouching`)
        (set `self.IsCrouching` false)))
    (:`then_1`
      (if (`self.IsAiming`)
        (set `self.IsAiming` false)))
    (:`then_2`
      (bind _output_get (set `self.IsSprinting` IsSprinting))
      (`self.F_SetSprintSpeed` _output_get))))

(fn `IF_GetAmmoInfo`
  (returns (TotalAmmo :type Integer) (BulletsInMag :type Integer))
  (bind _equipedweapon (`/Game/PropHunt/Blueprints/Characters/BP_WeaponsManager.EquipedWeapon` (`self.BP_WeaponsManager`)))
  (bind _asbp_firearm_weapon (cast `/Game/PropHunt/Blueprints/Weapons/BP_FirearmWeapon` _equipedweapon :!pure true))
  (`/Engine/EditorBlueprintResources/StandardMacros.IsValid` _equipedweapon
    (:`Is Valid`
      (return (`/Game/PropHunt/Blueprints/Weapons/BP_FirearmWeapon.Ammo` _asbp_firearm_weapon) (`/Game/PropHunt/Blueprints/Weapons/BP_FirearmWeapon.BulletsInMagazin` _asbp_firearm_weapon)))
    (:`Is Not Valid`
      (return 0 0))))

(fn `IF_GetEquipedWeapon`
  (returns (Weapon :type "Actor Object Reference"))
  (bind _bp_weaponsmanager (`self.BP_WeaponsManager`))
  (bind _equipedweapon (`/Game/PropHunt/Blueprints/Characters/BP_WeaponsManager.EquipedWeapon` _bp_weaponsmanager))
  (`/Engine/EditorBlueprintResources/StandardMacros.IsValid` _bp_weaponsmanager
    (:`Is Valid`
      (`/Engine/EditorBlueprintResources/StandardMacros.IsValid` _equipedweapon
        (:`Is Valid`
          (return _equipedweapon))
        (:`Is Not Valid`
          _)))
    (:`Is Not Valid`
      _))
  (return null))

(fn `IF_GetFollowCamera`
  (returns (Camera :type "CameraComponent Object Reference"))
  (return (`self.FollowCamera`)))

(fn `IF_GetHealth`
  (returns (Health :type "Float (double-precision)"))
  (return (`/Game/PropHunt/Blueprints/Characters/BP_HealthManager.Health` (`self.BP_HealthManager`))))

(fn `IF_GetTeam`
  (returns (Team :type Integer))
  (bind _team (message `/Game/PropHunt/Blueprints/Interfaces/BP_I_TeamPlayer.IF_GetTeam` (`self.PlayerState`)))
  (return _team))

(fn `IF_IsDead`
  (returns (IsDead :type Boolean))
  (return (`self.IsDead`)))

(fn `IF_SetHealth`
  (params (NewHealth :type "Float (double-precision)"))
  (returns (Health :type "Float (double-precision)"))
  (bind _output_get (set `/Game/PropHunt/Blueprints/Characters/BP_HealthManager.Health` NewHealth (`self.BP_HealthManager`)))
  (return _output_get))

(fn `IF_SetTeam`
  (params (NewTeam :type Integer))
  (returns (Team :type Integer))
  (bind _team (message `/Game/PropHunt/Blueprints/Interfaces/BP_I_TeamPlayer.IF_SetTeam` (`self.PlayerState`) NewTeam))
  (return _team))

(fn `OnRep_IsDead`
  (`/Engine/EditorBlueprintResources/ActorMacros.Switch Has Authority`
    (:`Authority`
      (bind _asbp_kernel_ps (cast `/Game/PropHunt/Blueprints/Kernel/BP_Kernel_PS` (`self.PlayerState`)))
      (set `/Game/PropHunt/Blueprints/Kernel/BP_Kernel_PS.IsDead` (`self.IsDead`) _asbp_kernel_ps))))

(fn `UserConstructionScript`)