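; Prop Hunt HUD class that owns the player's UMG screens, from loading, hunter wait and prop hide timer to finish screens, kill feed and chat.
; BeginPlay shows widgets for the current game state, then binds to game state dispatchers for phase changes, kill feed and chat updates.
; Phase changes clear the main widgets before showing new ones, with round start choosing by team.
; Toggle functions lazily create and cache each widget.
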(event `E_OnGameStartDelay`
  ;[1 1 1] Show loading screen
  (`self.F_RemoveAll`)
  (`self.F_ToggleLoadingScreen` true))

(event `E_OnRoundStart`
  ;[1 1 1] Round start - show wait screen for hunters
  (`self.F_RemoveAll`)
  (`KismetSystemLibrary.Delay` 1.0)
  (bind _team (message `/Game/PropHunt/Blueprints/Interfaces/BP_I_TeamPlayer.IF_GetTeam` (`GameplayStatics.GetPlayerController` 0)))
  (switch `int` _team
    (:`0`
      (`self.F_ToggleHunterWaitScreen` true))
    (:`1`
      (`self.F_TogglePropHideTimer` true)
      (`self.F_TogglePlayerHud` true))))

(event `self.ReceiveBeginPlay`
  (`/Engine/EditorBlueprintResources/StandardMacros.IsValid` (`GameplayStatics.GetGameState`)
    (:`Is Valid`
      _)
    (:`Is Not Valid`
      (`KismetSystemLibrary.Delay` 1.0)))
  (`|ExecutionSequence`
    (:`then_0`
      ;[1 1 1] Define what widget to show on begin play
      (`|ExecutionSequence`
        (:`then_0`
          (`self.F_RemoveAll`))
        (:`then_1`
          (switch `/Game/PropHunt/Blueprints/Kernel/E_GlobalState` (`/Game/PropHunt/Blueprints/Kernel/BP_Kernel_GS.GlobalState` (`/Game/PropHunt/Blueprints/Helpers/BP_Helpers.H_KernelGS`))
            (:`NewEnumerator23`
              (`self.F_ToggleLoadingScreen` true))
            (:`NewEnumerator28`
              (bind _team (message `/Game/PropHunt/Blueprints/Interfaces/BP_I_TeamPlayer.IF_GetTeam` (`self.PlayerOwner`)))
              (switch `int` _team
                (:`0`
                  (`self.F_ToggleHunterWaitScreen` true))
                (:`1`
                  (`self.F_TogglePropHideTimer` true)
                  (`self.F_TogglePlayerHud` true))))
            (:`NewEnumerator17`
              (`self.F_ToggleOserverHud` true))
            (:`NewEnumerator27`
              (`self.F_ToggleRoundFinishScreen` true))
            (:`NewEnumerator26`
              (`self.F_ToggleMatchFinishScreen` true))))))
    (:`then_1`
      ;[1 1 1] Show loading screen
      (add `/Game/PropHunt/Blueprints/Kernel/BP_Kernel_GS.D_GameStartDelay` (`/Game/PropHunt/Blueprints/Helpers/BP_Helpers.H_KernelGS`) (delegate `E_OnGameStartDelay`)))
    (:`then_2`
      ;[1 1 1] Round start - show wait screen for hunters
      (add `/Game/PropHunt/Blueprints/Kernel/BP_Kernel_GS.D_RoundStart` (`/Game/PropHunt/Blueprints/Helpers/BP_Helpers.H_KernelGS`) (delegate `E_OnRoundStart`)))
    (:`then_3`
      ;[1 1 1] Play time start - Show player hud and kill feed
      (add `/Game/PropHunt/Blueprints/Kernel/BP_Kernel_GS.D_PlayTime` (`/Game/PropHunt/Blueprints/Helpers/BP_Helpers.H_KernelGS`) (delegate `E_OnPlayTime`)))
    (:`then_4`
      ;[1 1 1] Round Finish - show round finish widget with winner name
      (add `/Game/PropHunt/Blueprints/Kernel/BP_Kernel_GS.D_RoundFinish` (`/Game/PropHunt/Blueprints/Helpers/BP_Helpers.H_KernelGS`) (delegate `E_OnRoundFinish`)))
    (:`then_5`
      ;[1 1 1] Match finish - how match finish widget with winner name
      (add `/Game/PropHunt/Blueprints/Kernel/BP_Kernel_GS.D_MatchFinish` (`/Game/PropHunt/Blueprints/Helpers/BP_Helpers.H_KernelGS`) (delegate `E_OnMatchFinish`)))
    (:`then_6`
      ;[1 1 1] Update kill feed
      (add `/Game/PropHunt/Blueprints/Kernel/BP_Kernel_GS.D_UpdateKillFeed` (`/Game/PropHunt/Blueprints/Helpers/BP_Helpers.H_KernelGS`) (delegate `E_UpdateKillFeed`)))
    (:`then_7`
      ;[1 1 1] Update game chat
      (add `/Game/PropHunt/Blueprints/Kernel/BP_Kernel_GS.D_UpdateGameChat` (`/Game/PropHunt/Blueprints/Helpers/BP_Helpers.H_KernelGS`) (delegate `E_UpdateGameChat`)))))

(event `E_OnPlayTime`
  ;[1 1 1] Play time start - Show player hud and kill feed
  (`self.F_RemoveAll`)
  (`self.F_TogglePlayerHud` true)
  (`self.F_ToggleKillFeed` true))

(event `E_ShowHitIndicator`
  (bind _playerhud (`self.PlayerHud`))
  ;[1 0 0.2682] Show and slowly hide enemy hit indicator
  (`/Engine/EditorBlueprintResources/StandardMacros.IsValid` _playerhud
    (:`Is Valid`
      (`/Game/PropHunt/Blueprints/Widgets/Game/BP_W_HUD.E_ActivateHitIndicator` _playerhud))))

(event `E_OnRoundFinish`
  ;[1 1 1] Round Finish - show round finish widget with winner name
  (`self.F_RemoveAll`)
  (`self.F_ToggleRoundFinishScreen` true))

(event `E_OnMatchFinish`
  ;[1 1 1] Match finish - how match finish widget with winner name
  (`self.F_RemoveAll`)
  (`self.F_ToggleMatchFinishScreen` true))

(event `E_UpdateKillFeed`
  (params (KillerId :type Integer) (VictimId :type Integer) (WeaponId :type Integer))
  (bind _killfeed (`self.KillFeed`))
  ;[1 1 1] Update kill feed
  (bind _returnvalue (`|CreateWidget` "/Game/PropHunt/Blueprints/Widgets/Game/BP_WE_KillFeedMessage.BP_WE_KillFeedMessage_C" (`self.PlayerOwner`) KillerId VictimId WeaponId))
  (`/Engine/EditorBlueprintResources/StandardMacros.IsValid` _killfeed
    (:`Is Valid`
      (`/Game/PropHunt/Blueprints/Widgets/Game/BP_W_KillFeed.E_AddMessage` _killfeed _returnvalue))
    (:`Is Not Valid`
      (`self.F_ToggleKillFeed` true)
      (`/Game/PropHunt/Blueprints/Widgets/Game/BP_W_KillFeed.E_AddMessage` (`self.KillFeed`) _returnvalue))))

(event `E_UpdateGameChat`
  (params (IsServer :type Boolean) (SenderId :type Integer) (Message :type String))
  ;[1 1 1] Update game chat
  (`self.F_ToggleGameChat` true)
  (`/Game/PropHunt/Blueprints/Widgets/Chat/BP_W_GameChat.E_AddMessage` (`self.GameChat`) IsServer SenderId Message))

(fn `F_RemoveAll`
  (`|ExecutionSequence`
    (:`then_0`
      (bind _playerhud (`self.PlayerHud`)
        (:`then`
          (`Widget.RemoveFromParent` _playerhud)
          (set `self.PlayerHud` null))
        (:`else`)))
    (:`then_1`
      (bind _observerhudwb (`self.ObserverHudWB`)
        (:`then`
          (`Widget.RemoveFromParent` _observerhudwb)
          (set `self.ObserverHudWB` null))
        (:`else`)))
    (:`then_2`
      (bind _killfeed (`self.KillFeed`)
        (:`then`
          (`Widget.RemoveFromParent` _killfeed)
          (set `self.KillFeed` null))
        (:`else`)))
    (:`then_3`
      (bind _matchfinishscreen (`self.MatchFinishScreen`)
        (:`then`
          (`Widget.RemoveFromParent` _matchfinishscreen)
          (set `self.MatchFinishScreen` null))
        (:`else`)))
    (:`then_4`
      (bind _killfeed_2 (`self.KillFeed`)
        (:`then`
          (`Widget.RemoveFromParent` _killfeed_2)
          (set `self.KillFeed` null))
        (:`else`)))
    (:`then_5`
      (bind _hunterwaitscreen (`self.HunterWaitScreen`)
        (:`then`
          (`Widget.RemoveFromParent` _hunterwaitscreen)
          (set `self.HunterWaitScreen` null))
        (:`else`)))
    (:`then_6`
      (bind _roundfinishscreen (`self.RoundFinishScreen`)
        (:`then`
          (`Widget.RemoveFromParent` _roundfinishscreen)
          (set `self.RoundFinishScreen` null))
        (:`else`)))
    (:`then_7`
      (bind _prophidetimer (`self.PropHideTimer`)
        (:`then`
          (`Widget.RemoveFromParent` _prophidetimer)
          (set `self.PropHideTimer` null))
        (:`else`)))
    (:`then_8`
      (bind _loadingscreen (`self.LoadingScreen`)
        (:`then`
          (`Widget.RemoveFromParent` _loadingscreen)
          (set `self.LoadingScreen` null))
        (:`else`)))
    (:`then_9`
      (bind _gamechat (`self.GameChat`)
        (:`then`
          (`Widget.RemoveFromParent` _gamechat)
          (set `self.GameChat` null))
        (:`else`)))))

(fn `F_ShowScoreNotify`
  (params (Score :type String) (Message :type String))
  (`|ExecutionSequence`
    (:`then_0`
      (bind _scorenotify (`self.ScoreNotify`)
        (:`then`
          (`Widget.RemoveFromParent` _scorenotify))
        (:`else`)))
    (:`then_1`
      (bind _returnvalue (`|CreateWidget` "/Game/PropHunt/Blueprints/Widgets/Game/BP_W_ScoreNotify.BP_W_ScoreNotify_C" (`self.PlayerOwner`) Score Message))
      (bind _output_get (set `self.ScoreNotify` _returnvalue))
      (`UserWidget.AddToViewport` _output_get 100))))

(fn `F_ToggleGameChat`
  (params (Show :type Boolean))
  (bind _gamechat (`self.GameChat`))
  (if Show
    (`self.GameChat`
      (:`then`
        (`/Game/PropHunt/Blueprints/Helpers/BP_MacroHelpers.MH_IsWidgetVisible` _gamechat
          (:`false`
            (`UserWidget.AddToViewport` _gamechat 0))))
      (:`else`
        (bind _returnvalue (`|CreateWidget` "/Game/PropHunt/Blueprints/Widgets/Chat/BP_W_GameChat.BP_W_GameChat_C" (`self.PlayerOwner`)))
        (bind _output_get (set `self.GameChat` _returnvalue))
        (`UserWidget.AddToViewport` _output_get 0)))
    (else
      (bind _gamechat_2 (`self.GameChat`)
        (:`then`
          (`Widget.RemoveFromParent` _gamechat_2))
        (:`else`)))))

(fn `F_ToggleHelp`
  (params (Show :type Boolean))
  (bind _help (`self.Help`))
  (if Show
    (`self.Help`
      (:`then`
        (`/Game/PropHunt/Blueprints/Helpers/BP_MacroHelpers.MH_IsWidgetVisible` _help
          (:`false`
            (`UserWidget.AddToViewport` _help 100))))
      (:`else`
        (bind _returnvalue (`|CreateWidget` "/Game/PropHunt/Blueprints/Widgets/Game/BP_W_Help.BP_W_Help_C" (`self.PlayerOwner`)))
        (bind _output_get (set `self.Help` _returnvalue))
        (`UserWidget.AddToViewport` _output_get 100)))
    (else
      (bind _help_2 (`self.Help`)
        (:`then`
          (`Widget.RemoveFromParent` _help_2))
        (:`else`)))))

(fn `F_ToggleHunterWaitScreen`
  (params (Show :type Boolean))
  (bind _hunterwaitscreen (`self.HunterWaitScreen`))
  (if Show
    (`self.HunterWaitScreen`
      (:`then`
        (`/Game/PropHunt/Blueprints/Helpers/BP_MacroHelpers.MH_IsWidgetVisible` _hunterwaitscreen
          (:`false`
            (`UserWidget.AddToViewport` _hunterwaitscreen 0))))
      (:`else`
        (bind _returnvalue (`|CreateWidget` "/Game/PropHunt/Blueprints/Widgets/Game/BP_W_HunterWaitScreen.BP_W_HunterWaitScreen_C" (`self.PlayerOwner`)))
        (bind _output_get (set `self.HunterWaitScreen` _returnvalue))
        (`UserWidget.AddToViewport` _output_get 0)))
    (else
      (bind _hunterwaitscreen_2 (`self.HunterWaitScreen`)
        (:`then`
          (`Widget.RemoveFromParent` _hunterwaitscreen_2))
        (:`else`)))))

(fn `F_ToggleInGameMenu`
  (params (Show :type Boolean))
  (bind _ingamemenu (`self.InGameMenu`))
  (if Show
    (`self.InGameMenu`
      (:`then`
        (`/Game/PropHunt/Blueprints/Helpers/BP_MacroHelpers.MH_IsWidgetVisible` _ingamemenu
          (:`false`
            (`UserWidget.AddToViewport` _ingamemenu 99))))
      (:`else`
        (bind _returnvalue (`|CreateWidget` "/Game/PropHunt/Blueprints/Widgets/Game/BP_W_InGameMenu.BP_W_InGameMenu_C" (`self.PlayerOwner`)))
        (bind _output_get (set `self.InGameMenu` _returnvalue))
        (`UserWidget.AddToViewport` _output_get 99)))
    (else
      (bind _ingamemenu_2 (`self.InGameMenu`)
        (:`then`
          (`Widget.RemoveFromParent` _ingamemenu_2))
        (:`else`)))))

(fn `F_ToggleKillFeed`
  (params (Show :type Boolean))
  (bind _killfeed (`self.KillFeed`))
  (if Show
    (`self.KillFeed`
      (:`then`
        (`/Game/PropHunt/Blueprints/Helpers/BP_MacroHelpers.MH_IsWidgetVisible` _killfeed
          (:`false`
            (`UserWidget.AddToViewport` _killfeed 0))))
      (:`else`
        (bind _returnvalue (`|CreateWidget` "/Game/PropHunt/Blueprints/Widgets/Game/BP_W_KillFeed.BP_W_KillFeed_C" (`self.PlayerOwner`)))
        (bind _output_get (set `self.KillFeed` _returnvalue))
        (`UserWidget.AddToViewport` _output_get 0)))
    (else
      (bind _killfeed_2 (`self.KillFeed`)
        (:`then`
          (`Widget.RemoveFromParent` _killfeed_2))
        (:`else`)))))

(fn `F_ToggleLoadingScreen`
  (params (Show :type Boolean))
  (bind _loadingscreen (`self.LoadingScreen`))
  (if Show
    (`self.LoadingScreen`
      (:`then`
        (`/Game/PropHunt/Blueprints/Helpers/BP_MacroHelpers.MH_IsWidgetVisible` _loadingscreen
          (:`false`
            (`UserWidget.AddToViewport` _loadingscreen 0))))
      (:`else`
        (bind _returnvalue (`|CreateWidget` "/Game/PropHunt/Blueprints/Widgets/Game/BP_W_LoadingScreen.BP_W_LoadingScreen_C" (`self.PlayerOwner`) (`KismetMathLibrary.Conv_IntToDouble` (`/Game/PropHunt/Blueprints/Kernel/BP_Kernel_GS.GameStartDelayS` (`/Game/PropHunt/Blueprints/Helpers/BP_Helpers.H_KernelGS`)))))
        (bind _output_get (set `self.LoadingScreen` _returnvalue))
        (`UserWidget.AddToViewport` _output_get 0)))
    (else
      (bind _loadingscreen_2 (`self.LoadingScreen`)
        (:`then`
          (`Widget.RemoveFromParent` _loadingscreen_2))
        (:`else`)))))

(fn `F_ToggleMatchFinishScreen`
  (params (Show :type Boolean))
  (bind _matchfinishscreen (`self.MatchFinishScreen`))
  (if Show
    (`self.MatchFinishScreen`
      (:`then`
        (`/Game/PropHunt/Blueprints/Helpers/BP_MacroHelpers.MH_IsWidgetVisible` _matchfinishscreen
          (:`false`
            (`UserWidget.AddToViewport` _matchfinishscreen 0))))
      (:`else`
        (bind _returnvalue (`|CreateWidget` "/Game/PropHunt/Blueprints/Widgets/Game/BP_W_MatchFinishScreen.BP_W_MatchFinishScreen_C" (`self.PlayerOwner`)))
        (bind _output_get (set `self.MatchFinishScreen` _returnvalue))
        (`UserWidget.AddToViewport` _output_get 0)))
    (else
      (bind _matchfinishscreen_2 (`self.MatchFinishScreen`)
        (:`then`
          (`Widget.RemoveFromParent` _matchfinishscreen_2))
        (:`else`)))))

(fn `F_ToggleOserverHud`
  (params (Show :type Boolean) (KillerId :type Integer))
  (returns (NewParam :type Boolean))
  (locals (killerNameLoc :type String))
  (bind _observerhudwb (`self.ObserverHudWB`))
  (if Show
    (`self.ObserverHudWB`
      (:`then`
        (`/Game/PropHunt/Blueprints/Helpers/BP_MacroHelpers.MH_IsWidgetVisible` _observerhudwb
          (:`false`
            (`UserWidget.AddToViewport` _observerhudwb 0))))
      (:`else`
        (bind _returnvalue (`|CreateWidget` "/Game/PropHunt/Blueprints/Widgets/Game/BP_W_ObserverHud.BP_W_ObserverHud_C" (`self.PlayerOwner`) KillerId))
        (bind _output_get (set `self.ObserverHudWB` _returnvalue))
        (`UserWidget.AddToViewport` _output_get 0)))
    (else
      (bind _observerhudwb_2 (`self.ObserverHudWB`)
        (:`then`
          (`Widget.RemoveFromParent` _observerhudwb_2)
          (return false))
        (:`else`)))))

(fn `F_TogglePlayerHud`
  (params (Show :type Boolean))
  (bind _playerhud (`self.PlayerHud`))
  (if Show
    (`self.PlayerHud`
      (:`then`
        (`/Game/PropHunt/Blueprints/Helpers/BP_MacroHelpers.MH_IsWidgetVisible` _playerhud
          (:`false`
            (`UserWidget.AddToViewport` _playerhud 0))))
      (:`else`
        (bind _returnvalue (`|CreateWidget` "/Game/PropHunt/Blueprints/Widgets/Game/BP_W_HUD.BP_W_HUD_C" (`self.PlayerOwner`)))
        (bind _output_get (set `self.PlayerHud` _returnvalue))
        (`UserWidget.AddToViewport` _output_get 0)))
    (else
      (bind _playerhud_2 (`self.PlayerHud`)
        (:`then`
          (`Widget.RemoveFromParent` _playerhud_2))
        (:`else`)))))

(fn `F_TogglePropHideTimer`
  (params (Show :type Boolean))
  (bind _prophidetimer (`self.PropHideTimer`))
  (if Show
    (`self.PropHideTimer`
      (:`then`
        (`/Game/PropHunt/Blueprints/Helpers/BP_MacroHelpers.MH_IsWidgetVisible` _prophidetimer
          (:`false`
            (`UserWidget.AddToViewport` _prophidetimer 0))))
      (:`else`
        (bind _returnvalue (`|CreateWidget` "/Game/PropHunt/Blueprints/Widgets/Game/BP_W_PropHideTimer.BP_W_PropHideTimer_C" (`self.PlayerOwner`)))
        (bind _output_get (set `self.PropHideTimer` _returnvalue))
        (`UserWidget.AddToViewport` _output_get 0)))
    (else
      (bind _prophidetimer_2 (`self.PropHideTimer`)
        (:`then`
          (`Widget.RemoveFromParent` _prophidetimer_2))
        (:`else`)))))

(fn `F_ToggleRoundFinishScreen`
  (params (Show :type Boolean))
  (bind _roundfinishscreen (`self.RoundFinishScreen`))
  (if Show
    (`self.RoundFinishScreen`
      (:`then`
        (`/Game/PropHunt/Blueprints/Helpers/BP_MacroHelpers.MH_IsWidgetVisible` _roundfinishscreen
          (:`false`
            (`UserWidget.AddToViewport` _roundfinishscreen 0))))
      (:`else`
        (bind _returnvalue (`|CreateWidget` "/Game/PropHunt/Blueprints/Widgets/Game/BP_W_RoundFinishScreen.BP_W_RoundFinishScreen_C" (`self.PlayerOwner`)))
        (bind _output_get (set `self.RoundFinishScreen` _returnvalue))
        (`UserWidget.AddToViewport` _output_get 0)))
    (else
      (bind _roundfinishscreen_2 (`self.RoundFinishScreen`)
        (:`then`
          (`Widget.RemoveFromParent` _roundfinishscreen_2))
        (:`else`)))))

(fn `F_ToggleScoreBoard`
  (params (Show :type Boolean))
  (bind _scoreboard (`self.Scoreboard`))
  (if Show
    (`self.Scoreboard`
      (:`then`
        (`/Game/PropHunt/Blueprints/Helpers/BP_MacroHelpers.MH_IsWidgetVisible` _scoreboard
          (:`false`
            (`UserWidget.AddToViewport` _scoreboard 100))))
      (:`else`
        (bind _returnvalue (`|CreateWidget` "/Game/PropHunt/Blueprints/Widgets/Scoreboard/BP_W_ScoreBoard.BP_W_ScoreBoard_C" (`self.PlayerOwner`)))
        (bind _output_get (set `self.Scoreboard` _returnvalue))
        (`UserWidget.AddToViewport` _output_get 100)))
    (else
      (bind _scoreboard_2 (`self.Scoreboard`)
        (:`then`
          (`Widget.RemoveFromParent` _scoreboard_2))
        (:`else`)))))

(fn `UserConstructionScript`)