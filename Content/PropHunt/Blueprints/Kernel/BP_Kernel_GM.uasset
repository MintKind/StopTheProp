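; Server game mode for a prop hunt match that manages hunter and prop teams, spawning, deaths and match settings.
; Settings come from the game instance or dedicated-server command line, initialized from both BeginPlay and PostLogin to work around early login.
; New players join the smaller team, then spawn or observe by round state.
; Kernel game state round events drive spawning, pawn cleanup and team swaps; deaths and logouts check for an early finish.
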(event `E_InitSettings`
  ;[1 0.5159 0.0913] INIT SETTINGS
  (if (not (`self.WasInitSettingsSet`))
    (`|ExecutionSequence`
      (:`then_0`
        (if (`KismetSystemLibrary.IsDedicatedServer`)
          (`self.FS_SetGameModeSettingsForDedicatedServer`)
          (else
            ;;[1 1 1 1 15] Get host game settings from MainGI
            (`self.FS_SetHostGameSettings`)))
        ;;[1 1 1] Check and set some default values to avoid errors
        (`self.F_CheckHostSettings`))
      (:`then_1`
        (`self.FS_GenerateTeamsArray`))
      (:`then_2`
        (set `self.WasInitSettingsSet` true)))))

(event `self.K2_PostLogin`
  (params (NewPlayer :type "PlayerController Object Reference"))
  ;[0 0.1238 1] LogIn event.
  ; Since OnPostLogin event can be called before BeginPlay event (issue UE-27284), I set "init settings" also in OnPostLogin event to be sure all settings was set right
  (`|ExecutionSequence`
    (:`then_0`
      (`self.E_InitSettings`))
    (:`then_1`
      (`self.FS_OnPostLogin` NewPlayer)
      (`KismetSystemLibrary.Delay` 0.5)
      (`self.FS_DefineWhatToDoWithPlayer` NewPlayer))))

(event `EA_RoundStart`
  ;[1 1 1] Round start - spawn all players
  (`|ExecutionSequence`
    (:`then_0`
      (switch `/Game/PropHunt/Blueprints/Kernel/E_GameMode` (`self.GameMode`)
        (:`NewEnumerator0`
          (if (not (`/Game/PropHunt/Blueprints/Kernel/BP_Kernel_GS.F_IsFirstRound` (`/Game/PropHunt/Blueprints/Helpers/BP_Helpers.H_KernelGS`)))
            (`self.FS_SwapTeams`)))))
    (:`then_1`
      (`self.FS_SpawnAllPlayers`))))

(event `self.ReceiveBeginPlay`
  ;[1 0 0] BEGIN PLAY
  (`|ExecutionSequence`
    (:`then_0`
      (`/Engine/EditorBlueprintResources/StandardMacros.IsValid` (`/Game/PropHunt/Blueprints/Helpers/BP_Helpers.H_KernelGS`)
        (:`Is Valid`
          _)
        (:`Is Not Valid`
          (`KismetSystemLibrary.Delay` 0.2)))
      (`|ExecutionSequence`
        (:`then_0`
          ;[1 1 1] Round start - spawn all players
          (add `/Game/PropHunt/Blueprints/Kernel/BP_Kernel_GS.D_RoundStart` (`/Game/PropHunt/Blueprints/Helpers/BP_Helpers.H_KernelGS`) (delegate `EA_RoundStart`)))
        (:`then_1`
          ;[1 1 1] round finish - destroy all players
          (add `/Game/PropHunt/Blueprints/Kernel/BP_Kernel_GS.D_RoundFinish` (`/Game/PropHunt/Blueprints/Helpers/BP_Helpers.H_KernelGS`) (delegate `EA_FinishRound`)))
        (:`then_2`
          ;[1 0 0] Match finish - swap teams
          (add `/Game/PropHunt/Blueprints/Kernel/BP_Kernel_GS.D_MatchFinish` (`/Game/PropHunt/Blueprints/Helpers/BP_Helpers.H_KernelGS`) (delegate `E_FinishMatch`)))))
    (:`then_1`
      (`self.E_InitSettings`))))

(event `self.K2_OnLogout`
  (params (ExitingController :type "Controller Object Reference"))
  (bind _kernelgs (`/Game/PropHunt/Blueprints/Helpers/BP_Helpers.H_KernelGS`))
  ;[0 0.1238 1] LogOut event. Update session info
  (`self.FS_OnLogout` ExitingController)
  (`KismetSystemLibrary.Delay` 1.0)
  (if (<= (`/Game/PropHunt/Blueprints/Kernel/BP_Kernel_GS.FS_GetTotalAliveTeams` (`/Game/PropHunt/Blueprints/Helpers/BP_Helpers.H_KernelGS`)) 1)
    (`/Game/PropHunt/Blueprints/Kernel/BP_Kernel_GS.FS_UpdateTeamScore` _kernelgs)
    (`/Game/PropHunt/Blueprints/Kernel/BP_Kernel_GS.EA_FinishMatch` _kernelgs)))

(event `EA_FinishRound`
  ;[1 1 1] round finish - destroy all players
  (`self.FS_DestroyAllPlayers`))

(event `E_FinishMatch`
  ;[1 0 0] Match finish - swap teams
  (`self.FS_DestroyAllPlayers`)
  (`self.FS_SwapTeams`))

(fn `F_CheckHostSettings`
  (`|ExecutionSequence`
    (:`then_0`
      (`/Game/PropHunt/Blueprints/Helpers/BP_MacroHelpers.MH_IsEmptyString` (`self.ServerName`)
        (:`true`
          (set `self.ServerName` "Unnamed Server"))))
    (:`then_1`
      (if (== (`self.MaxPlayers`) 0)
        (set `self.MaxPlayers` 16)))
    (:`then_2`
      (if (<= (`self.TotalRounds`) 1)
        (set `self.TotalRounds` 5)))))

(fn `FS Get RandomLocation`
  (params (SpawnPoints :type "Array of /Game/PropHunt/Blueprints/Kernel/BP_SpawnPoint Object Reference"))
  (returns (SpawnLocation :type "Transform Structure (by ref)"))
  (bind _output (`|GetArrayItem` SpawnPoints (`KismetMathLibrary.RandomInteger` (- (`KismetArrayLibrary.Array_Length` SpawnPoints) 1))))
  (`/Engine/EditorBlueprintResources/StandardMacros.IsValid` _output
    (:`Is Valid`
      (return (`self.GetTransform` _output)))
    (:`Is Not Valid`
      (return (`KismetMathLibrary.MakeTransform` (0.0 0.0 300.0))))))

(fn `FS_CanFinishRoundOnPlayerDeath`
  (returns (FinishRound :type Boolean))
  (return (<= (`/Game/PropHunt/Blueprints/Kernel/BP_Kernel_GS.FS_GetTotalAliveTeams` (`/Game/PropHunt/Blueprints/Helpers/BP_Helpers.H_KernelGS`)) 1)))

(fn `FS_DefineWhatToDoWithPlayer`
  (params (PC :type "PlayerController Object Reference"))
  (locals (PC_L :type "PlayerController Object Reference") (Team_L :type Integer :default 0))
  (bind _output_get (set `local.PC_L` PC))
  (bind _team (message `/Game/PropHunt/Blueprints/Interfaces/BP_I_TeamPlayer.IF_GetTeam` _output_get))
  (set `local.Team_L` _team)
  (switch `/Game/PropHunt/Blueprints/Kernel/E_GlobalState` (`/Game/PropHunt/Blueprints/Kernel/BP_Kernel_GS.GlobalState` (`/Game/PropHunt/Blueprints/Helpers/BP_Helpers.H_KernelGS`))
    (:`NewEnumerator28`
      (`self.FS_RespawnPlayer` (`local.PC_L`) (`self.FS_GetSpawnLocation` (`local.Team_L`))))
    (:`NewEnumerator17`
      (bind _asbp_kernel_ps (cast `/Game/PropHunt/Blueprints/Kernel/BP_Kernel_PS` (`Controller.PlayerState` (`local.PC_L`))))
      (`/Game/PropHunt/Blueprints/Kernel/BP_Kernel_PS.FS_SpawnObserverPawn` _asbp_kernel_ps 0))))

(fn `FS_DestroyAllPlayers`
  (for _array_element (`self.ConnectedPlayers`)
    (message `/Game/PropHunt/Blueprints/Interfaces/BP_I_BasePlayerController.IE_DestroyControlledPawn` _array_element)))

(fn `FS_GenerateTeamsArray`
  (`KismetArrayLibrary.Array_Add` (`self.TeamsAndNumberOfPlayers`))
  (`KismetArrayLibrary.Array_Add` (`self.TeamsAndNumberOfPlayers`)))

(fn `FS_GetPawnClass`
  (params (PC :type "PlayerController Object Reference"))
  (returns (PawnClass :type "Character Class Reference"))
  (bind _team (message `/Game/PropHunt/Blueprints/Interfaces/BP_I_TeamPlayer.IF_GetTeam` (`Controller.PlayerState` PC)))
  (switch `int` _team
    (:`Default`
      _)
    (:`0`
      _)
    (:`1`
      (return "/Game/PropHunt/Blueprints/Characters/BP_PropCharacter.BP_PropCharacter_C")))
  (return "/Game/PropHunt/Blueprints/Characters/BP_HunterCharacter.BP_HunterCharacter_C"))

(fn `FS_GetSpawnLocation`
  (params (Team :type Integer))
  (returns (SpawnLocation :type "Transform Structure"))
  (locals (HuntersTeamSpawnPoints_L :type "Array of /Game/PropHunt/Blueprints/Kernel/BP_SpawnPoint Object Reference") (PropsTeamSpawnPoints_L :type "Array of /Game/PropHunt/Blueprints/Kernel/BP_SpawnPoint Object Reference"))
  (`|ExecutionSequence`
    (:`then_0`
      (bind _outactors (`GameplayStatics.GetAllActorsOfClass` "/Game/PropHunt/Blueprints/Kernel/BP_SpawnPoint.BP_SpawnPoint_C"))
      (for _array_element _outactors
        (switch `int` (`/Game/PropHunt/Blueprints/Kernel/BP_SpawnPoint.Team` _array_element)
          (:`0`
            (`KismetArrayLibrary.Array_AddUnique` (`local.HuntersTeamSpawnPoints_L`) _array_element))
          (:`1`
            (`KismetArrayLibrary.Array_AddUnique` (`local.PropsTeamSpawnPoints_L`) _array_element)))))
    (:`then_1`
      (switch `int` Team
        (:`0`
          (return (`self.FS Get RandomLocation` (`local.HuntersTeamSpawnPoints_L`))))
        (:`1`
          (return (`self.FS Get RandomLocation` (`local.PropsTeamSpawnPoints_L`))))))))

(fn `FS_OnLogout`
  (params (ExitingController :type "Controller Object Reference"))
  (locals (ExitingPCLocal :type "PlayerController Object Reference"))
  (bind _asplayer_controller (cast `PlayerController` ExitingController))
  (set `local.ExitingPCLocal` _asplayer_controller)
  (`|ExecutionSequence`
    (:`then_0`
      (message `/Game/PropHunt/Blueprints/Interfaces/BP_I_BasePlayerController.IE_DisconnectFromTheServer` (`local.ExitingPCLocal`)))
    (:`then_1`
      ;[1 1 1] decrease players number in the exiting player's team
      (bind _team (message `/Game/PropHunt/Blueprints/Interfaces/BP_I_TeamPlayer.IF_GetTeam` (`Controller.PlayerState` (`local.ExitingPCLocal`))))
      (`self.FS_UpdateTeamsArray` _team))
    (:`then_2`
      (`KismetArrayLibrary.Array_RemoveItem` (`self.ConnectedPlayers`) (`local.ExitingPCLocal`))
      (set `local.ExitingPCLocal` null))))

(fn `FS_OnPostLogin`
  (params (NewPC :type "PlayerController Object Reference"))
  (locals (NewPC_L :type "PlayerController Object Reference"))
  (bind _output_get (set `local.NewPC_L` NewPC))
  (`|ExecutionSequence`
    (:`then_0`
      ;[1 1 1] disconnect new player if there is already maximim players on the server
      (if (`self.FS_ShouldDisconnectNewPlayer`)
        (message `/Game/PropHunt/Blueprints/Interfaces/BP_I_BasePlayerController.IE_DisconnectFromTheServer` (`local.NewPC_L`))
        (return)))
    (:`then_1`
      (`KismetArrayLibrary.Array_AddUnique` (`self.ConnectedPlayers`) _output_get)
      (`self.FS_SetTeamForNewPlayer` (`local.NewPC_L`)))))

(fn `FS_ProcessPlayerDeath`
  (params (VictimPS :type "PlayerState Object Reference") (KillerPS :type "PlayerState Object Reference") (WeaponId :type Integer))
  (locals (KillerPS_L :type "PlayerState Object Reference") (VictimPS_L :type "PlayerState Object Reference") (IsSuicide_L :type Boolean) (WeaponId_L :type Integer))
  (bind _playerid (`PlayerState.PlayerId` (`local.KillerPS_L`)))
  (set `local.VictimPS_L` VictimPS)
  (set `local.KillerPS_L` KillerPS)
  (set `local.WeaponId_L` WeaponId)
  (`|ExecutionSequence`
    (:`then_0`
      ;[1 1 1] Is suicide? When hunter shot in every prop
      (set `local.IsSuicide_L` (== (`local.KillerPS_L`) (`local.VictimPS_L`))))
    (:`then_1`
      ;[1 1 1] On death - spawn observer pawn and show observer hud for killed player
      (message `/Game/PropHunt/Blueprints/Interfaces/BP_I_PlayerStats.IE_UpdateDeaths` (`local.VictimPS_L`) (`PlayerState.PlayerId` (`local.KillerPS_L`))))
    (:`then_2`
      ;[1 1 1] update kills amount for killer player
      (message `/Game/PropHunt/Blueprints/Interfaces/BP_I_PlayerStats.IE_UpdateKills` (`local.KillerPS_L`))
      ;[1 1 1] Update score and send notify
      (message `/Game/PropHunt/Blueprints/Interfaces/BP_I_PlayerStats.IE_UpdateScore` (`local.KillerPS_L`) 100 "prop found"))
    (:`then_3`
      ;[1 1 1] Update kills log
      (if (`local.IsSuicide_L`)
        (`/Game/PropHunt/Blueprints/Kernel/BP_Kernel_GS.MC_UpdateKillFeed` (`/Game/PropHunt/Blueprints/Helpers/BP_Helpers.H_KernelGS`) _playerid _playerid (`local.WeaponId_L`))
        (else
          (`/Game/PropHunt/Blueprints/Kernel/BP_Kernel_GS.MC_UpdateKillFeed` (`/Game/PropHunt/Blueprints/Helpers/BP_Helpers.H_KernelGS`) (`PlayerState.PlayerId` (`local.KillerPS_L`)) (`PlayerState.PlayerId` (`local.VictimPS_L`)) (`local.WeaponId_L`)))))
    (:`then_4`
      ;[1 1 1] Finish play time if possible
      (if (`self.FS_CanFinishRoundOnPlayerDeath`)
        (`/Game/PropHunt/Blueprints/Kernel/BP_Kernel_GS.EA_FinishPlayTime` (`/Game/PropHunt/Blueprints/Helpers/BP_Helpers.H_KernelGS`))))))

(fn `FS_RespawnPlayer`
  (params (PC :type "PlayerController Object Reference") (RespawnLocation :type "Transform Structure"))
  (returns (RespawnedChar :type "Character Object Reference"))
  (locals (PC_L :type "PlayerController Object Reference") (RespawnLocation_L :type "Transform Structure"))
  (bind _output_get (set `local.PC_L` PC))
  (message `/Game/PropHunt/Blueprints/Interfaces/BP_I_BasePlayerController.IE_DestroyControlledPawn` _output_get)
  (bind _returnvalue (`|SpawnActorFromClass` (`self.FS_GetPawnClass` _output_get) RespawnLocation "AdjustIfPossibleButAlwaysSpawn" "OverrideRootScale" (`local.PC_L`) null))
  (`/Engine/EditorBlueprintResources/StandardMacros.IsValid` _returnvalue
    (:`Is Valid`
      (`Controller.Possess` (`local.PC_L`) _returnvalue)
      (return _returnvalue))
    (:`Is Not Valid`
      (`KismetSystemLibrary.PrintString` "RESPAWN ERROR" true true (struct :`R` 1.0 :`A` 1.0) 22.0))))

(fn `FS_SetGameModeSettingsForDedicatedServer`
  (locals (CommandLine :type String))
  (bind _returnvalue (`KismetSystemLibrary.GetCommandLine`))
  (set `local.CommandLine` _returnvalue)
  (`|ExecutionSequence`
    (:`then_0`
      ;[1 1 1] server name
      (set `self.ServerName` (`/Game/PropHunt/Blueprints/Helpers/BP_Helpers.H_ParseOption` (`local.CommandLine`) "sn")))
    (:`then_1`
      ;[1 1 1] map id
      (bind _returnvalue_2 (`GameplayStatics.GetCurrentLevelName` true))
      (switch `string` _returnvalue_2
        (:`ExampleMap`
          (set `self.MapId` 1))
        (:`TestMap`
          (set `self.MapId` 2))))
    (:`then_2`
      ;[1 1 1] max players
      (set `self.MaxPlayers` (`KismetStringLibrary.Conv_StringToInt` (`/Game/PropHunt/Blueprints/Helpers/BP_Helpers.H_ParseOption` (`local.CommandLine`) "mp"))))
    (:`then_3`
      ;[1 1 1] game mode
      (switch `string` (`/Game/PropHunt/Blueprints/Helpers/BP_Helpers.H_ParseOption` (`local.CommandLine`) "gm")
        (:`Default`
          (set `self.GameMode` "NewEnumerator0" :!label _label))
        (:`JFF`
          (goto _label))
        (:`CMP`
          (set `self.GameMode` "NewEnumerator1"))))
    (:`then_4`
      ;[1 1 1] total rounds
      (set `self.TotalRounds` (`KismetStringLibrary.Conv_StringToInt` (`/Game/PropHunt/Blueprints/Helpers/BP_Helpers.H_ParseOption` (`local.CommandLine`) "tr"))))))

(fn `FS_SetHostGameSettings`
  (bind _maingi (`/Game/PropHunt/Blueprints/Helpers/BP_Helpers.H_MainGI`))
  (set `self.ServerName` (`/Game/PropHunt/Blueprints/Kernel/BP_MainGI.ServerName` _maingi))
  (set `self.MapId` (`/Game/PropHunt/Blueprints/Kernel/BP_MainGI.MapId` _maingi))
  (set `self.MaxPlayers` (`/Game/PropHunt/Blueprints/Kernel/BP_MainGI.MaxPlayers` _maingi))
  (set `self.GameMode` (`/Game/PropHunt/Blueprints/Kernel/BP_MainGI.GameMode` _maingi))
  (set `self.TotalRounds` (`/Game/PropHunt/Blueprints/Kernel/BP_MainGI.TotalRounds` _maingi)))

(fn `FS_SetTeamForNewPlayer`
  (params (PC :type "PlayerController Object Reference"))
  (locals (PC_L :type "PlayerController Object Reference") (TeamToUpdate_L :type Integer) (CurrentTeam_L :type Integer) (NextTeam_L :type Integer))
  (set `local.PC_L` PC)
  ;[1 1 1] find team with minimal amount of players and set that team for new player
  (bind _team (message `/Game/PropHunt/Blueprints/Interfaces/BP_I_TeamPlayer.IF_SetTeam` (`Controller.PlayerState` (`local.PC_L`)) (`KismetMathLibrary.MinOfIntArray` (`self.TeamsAndNumberOfPlayers`))))
  (`self.FS_UpdateTeamsArray` _team true))

(fn `FS_ShouldDisconnectNewPlayer`
  (returns (ReturnValue :type Boolean))
  (return (>= (`/Game/PropHunt/Blueprints/Kernel/BP_Kernel_GS.F_GetTotalPlayers` (`/Game/PropHunt/Blueprints/Helpers/BP_Helpers.H_KernelGS`)) (`self.MaxPlayers`))))

(fn `FS_SpawnAllPlayers`
  (for _array_element (`self.ConnectedPlayers`)
    (bind _team (message `/Game/PropHunt/Blueprints/Interfaces/BP_I_TeamPlayer.IF_GetTeam` _array_element))
    (`self.FS_RespawnPlayer` _array_element (`self.FS_GetSpawnLocation` _team))))

(fn `FS_SwapTeams`
  (for _array_element (`GameStateBase.PlayerArray` (`GameplayStatics.GetGameState`))
    (bind _team (message `/Game/PropHunt/Blueprints/Interfaces/BP_I_TeamPlayer.IF_GetTeam` _array_element))
    (switch `int` _team
      (:`0`
        (`self.FS_UpdateTeamsArray` 0)
        (bind _team_2 (message `/Game/PropHunt/Blueprints/Interfaces/BP_I_TeamPlayer.IF_SetTeam` _array_element 1))
        (`self.FS_UpdateTeamsArray` _team_2 true))
      (:`1`
        (`self.FS_UpdateTeamsArray` 1)
        (bind _team_3 (message `/Game/PropHunt/Blueprints/Interfaces/BP_I_TeamPlayer.IF_SetTeam` _array_element 0))
        (`self.FS_UpdateTeamsArray` _team_3 true)))))

(fn `FS_UpdateTeamsArray`
  (params (Team :type Integer) (Add :type Boolean))
  (locals (Team_L :type Integer))
  (bind _teamsandnumberofplayers (`self.TeamsAndNumberOfPlayers`))
  (bind _teamsandnumberofplayers_2 (`self.TeamsAndNumberOfPlayers`))
  (bind _output (`|GetArrayItem` _teamsandnumberofplayers (`local.Team_L`)))
  (set `local.Team_L` Team)
  (if Add
    (`KismetArrayLibrary.Array_Set` _teamsandnumberofplayers_2 (`local.Team_L`) (+ (`|GetArrayItem` _teamsandnumberofplayers_2 (`local.Team_L`)) 1))
    (elif (not (<= _output 0))
      (`KismetArrayLibrary.Array_Set` _teamsandnumberofplayers (`local.Team_L`) (- _output 1)))))

(fn `UserConstructionScript`)