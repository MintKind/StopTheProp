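; Prop Hunt Game State that runs the match round cycle and tracks Hunters and Props scores.
; GlobalState's RepNotify restarts a one-second server countdown and multicasts the phase to event dispatchers; expiry advances the phase, and events can end play or match early.
; Alive-team checks decide winners, favoring Props when both survive, with round scores kept in Competitive mode.
; Multicasts also relay kill feed and chat.
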(event `MC_UpdateGameChat`
  (params (IsServer :type Boolean) (SenderId :type Integer) (Message :type String))
  ;[0 0.8709 1] Update game chat
  (`self.D_UpdateGameChat` IsServer SenderId Message))

(event `MC_UpdateKillFeed`
  (params (KillerId :type Integer) (VictimId :type Integer) (WeaponId :type Integer))
  ;[0 0.8709 1] Update kills log
  (`self.D_UpdateKillFeed` KillerId VictimId WeaponId))

(event `self.ReceiveBeginPlay`
  ;[1 0.7631 0] BEGIN PLAY
  (`self.F_SetTime`)
  (`/Engine/EditorBlueprintResources/ActorMacros.Switch Has Authority`
    (:`Authority`
      ;;[1 0 0] It starts main timer. OnRep_GlobalState.
      (set `self.GlobalState` "NewEnumerator23"))))

(event `EA_FinishPlayTime`
  ;[1 0 0.0759] Finish play time
  (`KismetSystemLibrary.Delay` 1.0)
  (`self.FS Define Next Global State`))

(event `EA_FinishMatch`
  ;[1 0 0.0759] Finish play time
  (`KismetSystemLibrary.Delay` 1.0)
  (set `self.GlobalState` "NewEnumerator26"))

(event `MC_OnGlobalStateChange`
  (params (NewGlobalState :type "/Game/PropHunt/Blueprints/Kernel/E_GlobalState Enum" :default "NewEnumerator23"))
  ;[1 0 0.3256] Multicast current state -> call event dispatcher on clients
  (switch `/Game/PropHunt/Blueprints/Kernel/E_GlobalState` NewGlobalState
    (:`NewEnumerator23`
      (`self.D_GameStartDelay`))
    (:`NewEnumerator28`
      (`self.D_RoundStart`))
    (:`NewEnumerator17`
      (`self.D_PlayTime`))
    (:`NewEnumerator27`
      (`self.D_RoundFinish`))
    (:`NewEnumerator26`
      (`self.D_MatchFinish`))))

(fn `F_GetAliveTeamPlayers`
  (params (Team :type Integer))
  (returns (AlivePlayers :type Integer))
  (locals (AlivePlayers_L :type Integer))
  (set `local.AlivePlayers_L` 0)
  (for _array_element (`self.PlayerArray`)
    (bind _asbp_kernel_ps (cast `/Game/PropHunt/Blueprints/Kernel/BP_Kernel_PS` _array_element))
    (bind _team (message `/Game/PropHunt/Blueprints/Interfaces/BP_I_TeamPlayer.IF_GetTeam` _asbp_kernel_ps))
    (if (and (not (`/Game/PropHunt/Blueprints/Kernel/BP_Kernel_PS.IsDead` _asbp_kernel_ps)) (== _team Team))
      (set `local.AlivePlayers_L` (+ (`local.AlivePlayers_L`) 1))))
  (return (`local.AlivePlayers_L`)))

(fn `F_GetTeamScore`
  (params (team :type Integer))
  (returns (TeamScore :type Integer))
  (switch `int` team
    (:`0`
      (return (`self.HuntersTeamScore`)))
    (:`1`
      (return (`self.PropsTeamScore`)))))

(fn `F_GetTotalAlivePlayers`
  (returns (TotalAlivePlayers :type Integer))
  (locals (AlivePlayers_L :type Integer))
  (set `local.AlivePlayers_L` 0)
  (for _array_element (`self.PlayerArray`)
    (bind _asbp_kernel_ps (cast `/Game/PropHunt/Blueprints/Kernel/BP_Kernel_PS` _array_element))
    (if (not (`/Game/PropHunt/Blueprints/Kernel/BP_Kernel_PS.IsDead` _asbp_kernel_ps))
      (set `local.AlivePlayers_L` (+ (`local.AlivePlayers_L`) 1))))
  (return (`local.AlivePlayers_L`)))

(fn `F_GetTotalPlayers`
  (returns (TotalPlayers :type Integer))
  (return (`KismetArrayLibrary.Array_Length` (`self.PlayerArray`))))

(fn `F_GetWinner`
  (returns (Winner :type String))
  (switch `/Game/PropHunt/Blueprints/Kernel/E_GameMode` (`/Game/PropHunt/Blueprints/Kernel/BP_MainGI.GameMode` (`/Game/PropHunt/Blueprints/Helpers/BP_Helpers.H_MainGI`))
    (:`NewEnumerator0`
      _)
    (:`NewEnumerator1`
      (if (`|EnumEquality` (`self.GlobalState`) "NewEnumerator26")
        (if (> (`self.HuntersTeamScore`) (`self.PropsTeamScore`))
          (return "HUNTERS")
          (elif (> (`self.PropsTeamScore`) (`self.HuntersTeamScore`))
            (return "PROPS")
            (else
              (return "DRAW"))))
        (else
          _))))
  (if (== (`self.FS_GetTotalAliveTeams`) 2)
    (return "PROPS")
    (else
      (switch `int` (`self.FS_FindLastAliveTeam`)
        (:`0`
          (return "HUNTERS"))
        (:`1`
          (return "PROPS"))))))

(fn `F_IsFirstRound`
  (returns (IsLastRound :type Boolean))
  (return (== (`self.RoundsLeft`) (`/Game/PropHunt/Blueprints/Kernel/BP_Kernel_GM.TotalRounds` (`/Game/PropHunt/Blueprints/Helpers/BP_Helpers.H_KernelGM`)))))

(fn `F_IsLastRound`
  (returns (IsLastRound :type Boolean))
  (return (<= (`self.RoundsLeft`) 0)))

(fn `F_SetTime`
  (set `self.GameStartDelayS` 2)
  (set `self.RoundStartTimeS` 30)
  (set `self.PlayTimeS` 360)
  (set `self.RoundFinishTimeS` 5)
  (set `self.MatchFinishTimeS` 10))

(fn `FS Define Next Global State`
  (switch `/Game/PropHunt/Blueprints/Kernel/E_GlobalState` (`self.GlobalState`)
    (:`NewEnumerator23`
      (`self.FS_ResetStats`)
      (set `self.GlobalState` "NewEnumerator28"))
    (:`NewEnumerator28`
      (set `self.GlobalState` "NewEnumerator17"))
    (:`NewEnumerator17`
      (`self.FS_UpdateTeamScore`)
      (set `self.RoundsLeft` (- (`self.RoundsLeft`) 1))
      (if (`self.F_IsLastRound`)
        (set `self.GlobalState` "NewEnumerator26")
        (else
          (set `self.GlobalState` "NewEnumerator27"))))
    (:`NewEnumerator27`
      (set `self.GlobalState` "NewEnumerator28"))
    (:`NewEnumerator26`
      (set `self.GlobalState` "NewEnumerator23"))))

(fn `FS_DecreaseTime`
  (returns (IsTimeOver :type Boolean))
  (bind _output_get (set `self.CurrentTime` (- (`self.CurrentTime`) 1)))
  (return (<= _output_get 0)))

(fn `FS_FindLastAliveTeam`
  (returns (TeamId :type Integer))
  (locals (LastAliveTeam_L :type Integer) (TotalAliveTeams_L :type Integer) (WasTeamFound :type Boolean))
  (bind _output (`|GetArrayItem` (`self.PlayerArray`)))
  (if (> (`self.F_GetAliveTeamPlayers` 0) 0)
    (return 0)
    (elif (> (`self.F_GetAliveTeamPlayers` 1) 0)
      (return 1)
      (else
        ;[1 1 1] if players left, just find player who is still on the server
        (`/Engine/EditorBlueprintResources/StandardMacros.IsValid` _output
          (:`Is Valid`
            (bind _team (message `/Game/PropHunt/Blueprints/Interfaces/BP_I_TeamPlayer.IF_GetTeam` _output))
            (return _team)))))))

(fn `FS_GetTotalAliveTeams`
  (returns (AliveTeamsNumber :type Integer))
  (locals (TotalAliveTeams_L :type Integer))
  (for (_ _array_index) (`self.PlayerArray`)
    (if (> (`self.F_GetAliveTeamPlayers` _array_index) 0)
      (set `local.TotalAliveTeams_L` (+ (`local.TotalAliveTeams_L`) 1))))
  (return (`local.TotalAliveTeams_L`)))

(fn `FS_MainTimer`
  (bind _istimeover (`self.FS_DecreaseTime`))
  (if _istimeover
    (`self.FS_StopMainTimer`)
    (`self.FS Define Next Global State`)))

(fn `FS_ResetStats`
  (set `self.HuntersTeamScore` 0)
  (set `self.PropsTeamScore` 0)
  (set `self.RoundsLeft` (`/Game/PropHunt/Blueprints/Kernel/BP_Kernel_GM.TotalRounds` (`/Game/PropHunt/Blueprints/Helpers/BP_Helpers.H_KernelGM`))))

(fn `FS_StartMainTimer`
  (params (NewTime :type Integer))
  (`/Engine/EditorBlueprintResources/ActorMacros.Switch Has Authority`
    (:`Authority`
      (`self.FS_StopMainTimer`)
      (set `self.CurrentTime` NewTime)
      (bind _returnvalue (`KismetSystemLibrary.K2_SetTimer` null "FS_MainTimer" 1.0 true))
      (set `self.MainTimer` _returnvalue))))

(fn `FS_StopMainTimer`
  (`KismetSystemLibrary.K2_ClearAndInvalidateTimerHandle` (`self.MainTimer`)))

(fn `FS_UpdateTeamScore`
  (switch `/Game/PropHunt/Blueprints/Kernel/E_GameMode` (`/Game/PropHunt/Blueprints/Kernel/BP_MainGI.GameMode` (`/Game/PropHunt/Blueprints/Helpers/BP_Helpers.H_MainGI`))
    (:`NewEnumerator1`
      (if (== (`self.FS_GetTotalAliveTeams`) 2)
        (set `self.PropsTeamScore` (+ (`self.PropsTeamScore`) 1))
        (else
          (switch `int` (`self.FS_FindLastAliveTeam`)
            (:`0`
              (set `self.HuntersTeamScore` (+ (`self.HuntersTeamScore`) 1)))
            (:`1`
              (set `self.PropsTeamScore` (+ (`self.PropsTeamScore`) 1)))))))))

(fn `OnRep_GlobalState`
  (`/Engine/EditorBlueprintResources/ActorMacros.Switch Has Authority`
    (:`Authority`
      (`self.FS_StopMainTimer`)
      (`self.MC_OnGlobalStateChange` (`self.GlobalState`))
      (switch `/Game/PropHunt/Blueprints/Kernel/E_GlobalState` (`self.GlobalState`)
        (:`NewEnumerator23`
          (`self.FS_StartMainTimer` (`self.GameStartDelayS`)))
        (:`NewEnumerator28`
          (`self.FS_StartMainTimer` (`self.RoundStartTimeS`)))
        (:`NewEnumerator17`
          (`self.FS_StartMainTimer` (`self.PlayTimeS`)))
        (:`NewEnumerator27`
          (`self.FS_StartMainTimer` (`self.RoundFinishTimeS`)))
        (:`NewEnumerator26`
          (`self.FS_StartMainTimer` (`self.MatchFinishTimeS`)))))))

(fn `UserConstructionScript`)