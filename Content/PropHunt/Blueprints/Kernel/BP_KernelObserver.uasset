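; Spectator actor for PropHunt that follows living hunter and prop characters, with left and right mouse clicks cycling targets.
; The server handles switching, gathering living characters through an interface death check and attaching to the target's "observer" mesh socket at its ObserverArrow transform.
; Server Tick detaches the observer in place when its target dies or becomes invalid.
; Without a valid target it moves above world origin, with a workaround for dedicated servers.
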(event `self.ReceiveBeginPlay`
  ;[1 1 1] Begin play
  (`/Engine/EditorBlueprintResources/ActorMacros.Switch Has Authority`
    (:`Authority`
      (`|ExecutionSequence`
        (:`then_0`
          (set `self.CurrentObservablePawnIndex` 0))
        (:`then_1`
          (`/Engine/EditorBlueprintResources/StandardMacros.IsValid` (`self.ObservableCharacter`)
            (:`Is Valid`
              (`KismetSystemLibrary.Delay` 1.5)
              (`self.FS_SetObservableCharacter` (`KismetArrayLibrary.Array_Find` (`self.FS_CollectAllAliveCharacters`) (`self.ObservableCharacter`))))
            (:`Is Not Valid`
              (`self.FS_TryToFindPawnToObserve`))))))))

(event `SRV_ChangeObservableCharacter`
  (params (Next :type Boolean))
  ;[1 1 1] Change observable player
  (if Next
    (`self.FS_WatchNextCharacter`)
    (else
      (`self.FS_WatchPreviousCharacter`))))

(event `Key|LeftMouseButton`
  (params (Key :type "Key Structure"))
  ;[1 1 1] Observe next player
  (:`Pressed`
    (`self.SRV_ChangeObservableCharacter` true)))

(event `Key|RightMouseButton`
  (params (Key :type "Key Structure"))
  ;[1 1 1] Observe previous player
  (:`Pressed`
    (`self.SRV_ChangeObservableCharacter` false)))

(event `self.ReceiveTick`
  (params (DeltaSeconds :type "Float (single-precision)"))
  (bind _observablecharacter (`self.ObservableCharacter`))
  ;[1 1 1] Tick. In case of current observable player death we need to find next one
  (`/Engine/EditorBlueprintResources/ActorMacros.Switch Has Authority`
    (:`Authority`
      (if (not (`self.IsDetached`))
        (`/Engine/EditorBlueprintResources/StandardMacros.IsValid` _observablecharacter
          (:`Is Valid`
            (bind _isdead (message `/Game/PropHunt/Blueprints/Interfaces/BP_I_BaseCharacter.IF_IsDead` _observablecharacter))
            (if _isdead
              (`self.K2_DetachFromActor` "KeepWorld" "KeepWorld" "KeepWorld" :!label _label)
              (set `self.IsDetached` true)))
          (:`Is Not Valid`
            (goto _label)))))))

(fn `FS_CollectAllAliveCharacters`
  (returns (AllCharacters :type "Array of Character Object Reference"))
  (bind _outactors (`GameplayStatics.GetAllActorsOfClass` "/Script/Engine.Character"))
  (for _array_element _outactors
    (bind _isdead (message `/Game/PropHunt/Blueprints/Interfaces/BP_I_BaseCharacter.IF_IsDead` _array_element))
    (if (not _isdead)
      (`KismetArrayLibrary.Array_AddUnique` (`self.AllCharacters`) _array_element)))
  (return (`self.AllCharacters`)))

(fn `FS_SetObservableCharacter`
  (params (Index :type Integer))
  (bind _output_get (set `self.CurrentObservablePawnIndex` Index))
  (set `self.IsDetached` false)
  (bind _output (`|GetArrayItem` (`self.FS_CollectAllAliveCharacters`) _output_get))
  (`/Engine/EditorBlueprintResources/StandardMacros.IsValid` _output
    (:`Is Valid`
      (set `self.ObservableCharacter` _output)
      (`self.K2_AttachToComponent` (`Character.Mesh` (`self.ObservableCharacter`)) "observer" "SnapToTarget" "KeepWorld" "KeepWorld" :!label _label)
      (bind _asbp_hunter_character (cast `/Game/PropHunt/Blueprints/Characters/BP_HunterCharacter` (`self.ObservableCharacter`))
        (:`then`
          (bind _observerarrow (`/Game/PropHunt/Blueprints/Characters/BP_HunterCharacter.ObserverArrow` _asbp_hunter_character))
          (`self.K2_SetActorLocation` (`SceneComponent.K2_GetComponentLocation` _observerarrow))
          (`self.K2_SetActorRotation` (`SceneComponent.K2_GetComponentRotation` _observerarrow)))
        (:`CastFailed`
          (bind _asbp_prop_character (cast `/Game/PropHunt/Blueprints/Characters/BP_PropCharacter` (`self.ObservableCharacter`)))
          (bind _observerarrow_2 (`/Game/PropHunt/Blueprints/Characters/BP_PropCharacter.ObserverArrow` _asbp_prop_character))
          (`self.K2_SetActorLocation` (`SceneComponent.K2_GetComponentLocation` _observerarrow_2))
          (`self.K2_SetActorRotation` (`SceneComponent.K2_GetComponentRotation` _observerarrow_2)))))
    (:`Is Not Valid`
      ;[1 1 1] somewhy default function doen't work on dedicated server. this is a fix
      (if (and (< (`self.GetGameTimeSinceCreation`) (+ (`self.GetGameTimeSinceCreation`) 1.0)) (`KismetSystemLibrary.IsValid` (`self.ObservableCharacter`)))
        (goto _label)
        (else
          (`self.FS_SpawnAtCenter`))))))

(fn `FS_SpawnAtCenter`
  (`self.K2_DetachFromActor` "KeepWorld" "KeepWorld" "KeepWorld")
  (`self.K2_SetActorLocation` (0.0 0.0 1000.0)))

(fn `FS_TryToFindPawnToObserve`
  (for (_array_element _array_index) (`self.FS_CollectAllAliveCharacters`)
    (bind _isdead (message `/Game/PropHunt/Blueprints/Interfaces/BP_I_BaseCharacter.IF_IsDead` _array_element))
    (if (not _isdead)
      (`|ExecutionSequence`
        (:`then_0`
          (break))
        (:`then_1`
          (`self.FS_SetObservableCharacter` _array_index)))))
  (`/Engine/EditorBlueprintResources/StandardMacros.IsValid` (`self.ObservableCharacter`)
    (:`Is Not Valid`
      (`self.FS_SpawnAtCenter`))))

(fn `FS_WatchNextCharacter`
  (locals (NextObservablePawnIndex_L :type Integer))
  (bind _returnvalue (+ (`self.CurrentObservablePawnIndex`) 1))
  (if (`KismetArrayLibrary.Array_IsValidIndex` (`self.FS_CollectAllAliveCharacters`) _returnvalue)
    (`self.FS_SetObservableCharacter` _returnvalue)
    (elif (`KismetArrayLibrary.Array_IsValidIndex` (`self.FS_CollectAllAliveCharacters`))
      (bind _output_get (set `self.CurrentObservablePawnIndex` 0))
      (`self.FS_SetObservableCharacter` _output_get))))

(fn `FS_WatchPreviousCharacter`
  (locals (PreviousObservablePawnIndex_L :type Integer))
  (bind _allcharacters (`self.FS_CollectAllAliveCharacters`))
  (bind _returnvalue (- (`self.CurrentObservablePawnIndex`) 1))
  (bind _returnvalue_2 (- (`KismetArrayLibrary.Array_Length` _allcharacters) 1))
  (if (`KismetArrayLibrary.Array_IsValidIndex` (`self.FS_CollectAllAliveCharacters`) _returnvalue)
    (`self.FS_SetObservableCharacter` _returnvalue)
    (elif (`KismetArrayLibrary.Array_IsValidIndex` _allcharacters _returnvalue_2)
      (`self.FS_SetObservableCharacter` _returnvalue_2))))

(fn `UserConstructionScript`)