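; Base-level PropHunt player controller handling UI input, chat, team access and disconnection.
; On BeginPlay, the local controller pulls host settings from the GameMode by server-to-client RPC and caches them in the GameInstance for UI.
; Keys toggle the menu, scoreboard and chat; messages relay through GameState multicast, while team interface calls forward to PlayerState.
; Disconnecting destroys the pawn server-side and returns to MainMenu; debug keys inspect names and teams or shorten the timer.
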(event `Key|N`
  (params (Key :type "Key Structure"))
  ;[1 1 1] TEst and debug finctions
  ;;[1 1 1] show name
  (:`Pressed`
    (`KismetSystemLibrary.PrintString` (`PlayerState.GetPlayerName` (`self.PlayerState`)))))

(event `Key|T`
  (params (Key :type "Key Structure"))
  ;[1 1 1] TEst and debug finctions
  ;;[1 1 1] Show my team id
  (:`Pressed`
    (bind _team (message `/Game/PropHunt/Blueprints/Interfaces/BP_I_TeamPlayer.IF_GetTeam` (`self.PlayerState`)))
    (`KismetSystemLibrary.PrintString` (`KismetStringLibrary.Conv_IntToString` _team))))

(event `Key|Add`
  (params (Key :type "Key Structure"))
  ;[1 1 1] TEst and debug finctions
  ;;[1 1 1] for testing. set current time = 2 seconds
  (:`Pressed`
    (`self.srv_5`)))

(event `Key|Four`
  (params (Key :type "Key Structure"))
  ;[1 1 1] TEst and debug finctions
  ;;[1 1 1] Show all teams
  (:`Pressed`
    (`self.SRV_Test`)))

(event `srv_5`
  ;[1 1 1] TEst and debug finctions
  ;;[1 1 1] for testing. set current time = 2 seconds
  (set `/Game/PropHunt/Blueprints/Kernel/BP_Kernel_GS.CurrentTime` 2 (`/Game/PropHunt/Blueprints/Helpers/BP_Helpers.H_KernelGS`)))

(event `SRV_Test`
  ;[1 1 1] TEst and debug finctions
  ;;[1 1 1] Show all teams
  (for (_array_element _array_index) (`/Game/PropHunt/Blueprints/Kernel/BP_Kernel_GM.TeamsAndNumberOfPlayers` (`/Game/PropHunt/Blueprints/Helpers/BP_Helpers.H_KernelGM`))
    (`KismetSystemLibrary.PrintString` (`KismetStringLibrary.Concat_StrStr` (`KismetStringLibrary.Concat_StrStr` "TEAM ID = " (`KismetStringLibrary.Conv_IntToString` _array_index)) (`KismetStringLibrary.Concat_StrStr` ";; PLAYERS = " (`KismetStringLibrary.Conv_IntToString` _array_element))) true true (struct :`G` 0.66 :`B` 1.0 :`A` 1.0) 22.0)))

(event `self.ReceiveBeginPlay`
  ;[1 1 1] Begin play. Load game setting from server - we need them for ui
  (if (`self.IsLocalPlayerController`)
    (`self.SRV_GetHostSettings`)))

(event `self.IE_DestroyControlledPawn`
  ;[1 1 1] Destroy character
  (`self.SRV_DestroyPawn`))

(event `SRV_DestroyPawn`
  (bind _returnvalue (`self.GetSpectatorPawn`))
  ;[1 1 1] Destroy character
  (`/Engine/EditorBlueprintResources/StandardMacros.IsValid` _returnvalue
    (:`Is Valid`
      (`self.K2_DestroyActor` _returnvalue))
    (:`Is Not Valid`
      _))
  (message `/Game/PropHunt/Blueprints/Interfaces/BP_I_BaseCharacter.IE_DestroySelf` (`self.K2_GetPawn`)))

(event `SRV_GetHostSettings`
  (bind _kernelgm (`/Game/PropHunt/Blueprints/Helpers/BP_Helpers.H_KernelGM`))
  ;[1 0 0.1247] Get host settings from server
  (`self.CL_SaveHostSettingsInLocalGI` (`/Game/PropHunt/Blueprints/Kernel/BP_Kernel_GM.ServerName` _kernelgm) (`/Game/PropHunt/Blueprints/Kernel/BP_Kernel_GM.MapId` _kernelgm) (`/Game/PropHunt/Blueprints/Kernel/BP_Kernel_GM.MaxPlayers` _kernelgm) (`/Game/PropHunt/Blueprints/Kernel/BP_Kernel_GM.GameMode` _kernelgm) (`/Game/PropHunt/Blueprints/Kernel/BP_Kernel_GM.TotalRounds` _kernelgm)))

(event `self.IE_DisconnectFromTheServer`
  ;[1 1 1] Disconnect
  (`self.IE_DestroyControlledPawn`)
  (`self.CL_Disconnect`))

(event `self.ReceiveEndPlay`
  (params (EndPlayReason :type "EEndPlayReason Enum" :default "Destroyed"))
  ;[1 1 1] Disconnect
  (`self.IE_DestroyControlledPawn`))

(event `CL_Disconnect`
  ;[1 1 1] Disconnect
  (`GameplayStatics.OpenLevel` "MainMenu")
  (`DestroySessionCallbackProxy.DestroySession` self))

(event `CL_SaveHostSettingsInLocalGI`
  (params (ServerName :type String) (MapId :type Integer) (MaxPlayers :type Integer) (GameMode :type "/Game/PropHunt/Blueprints/Kernel/E_GameMode Enum" :default "NewEnumerator0") (TotalRounds :type Integer))
  (bind _maingi (`/Game/PropHunt/Blueprints/Helpers/BP_Helpers.H_MainGI`))
  ;[1 0 0.1247] Save host settings in local GameInstance. We need them for UI
  (set `/Game/PropHunt/Blueprints/Kernel/BP_MainGI.ServerName` ServerName _maingi)
  (set `/Game/PropHunt/Blueprints/Kernel/BP_MainGI.MapId` MapId _maingi)
  (set `/Game/PropHunt/Blueprints/Kernel/BP_MainGI.MaxPlayers` MaxPlayers _maingi)
  (set `/Game/PropHunt/Blueprints/Kernel/BP_MainGI.GameMode` GameMode _maingi)
  (set `/Game/PropHunt/Blueprints/Kernel/BP_MainGI.TotalRounds` TotalRounds _maingi))

(event `SRV_SendChatMessage`
  (params (IsServer :type Boolean) (Message :type String))
  ;[0 0.6122 1] Send chat message
  (`/Game/PropHunt/Blueprints/Kernel/BP_Kernel_GS.MC_UpdateGameChat` (`/Game/PropHunt/Blueprints/Helpers/BP_Helpers.H_KernelGS`) IsServer (`PlayerState.PlayerId` (`self.PlayerState`)) Message))

(event `Key|Q`
  (params (Key :type "Key Structure"))
  ;[1 1 1] Show help info
)

(event `Key|Escape`
  (params (Key :type "Key Structure"))
  (bind _returnvalue (`GameplayStatics.GetPlayerCharacter` 0))
  (bind _returnvalue_2 (`GameplayStatics.GetPlayerCharacter` 0))
  ;[1 1 1] Show / hide in-game menu
  (:`Pressed`
    (bind _isa (`/Engine/EditorBlueprintResources/StandardMacros.FlipFlop` :!label _label)
      (:`A`
        (if _isa
          (`/Game/PropHunt/Blueprints/Kernel/BP_Kernel_HUD.F_ToggleInGameMenu` (`/Game/PropHunt/Blueprints/Helpers/BP_Helpers.H_KernelHUD`) true)
          (set `self.bShowMouseCursor` true)
          (`/Engine/EditorBlueprintResources/StandardMacros.IsValid` _returnvalue_2
            (:`Is Valid`
              (`self.DisableInput` _returnvalue_2 self)))))
      (:`B`
        (`/Game/PropHunt/Blueprints/Kernel/BP_Kernel_HUD.F_ToggleInGameMenu` (`/Game/PropHunt/Blueprints/Helpers/BP_Helpers.H_KernelHUD`) false)
        (set `PlayerController.bShowMouseCursor` false (`GameplayStatics.GetPlayerController` 0))
        (`/Engine/EditorBlueprintResources/StandardMacros.IsValid` _returnvalue
          (:`Is Valid`
            (`self.EnableInput` _returnvalue self)))))))

(event `Key|Z`
  (params (Key :type "Key Structure"))
  ;[1 1 1] Show / hide in-game menu
  (:`Pressed`
    (goto _label)))

(event `Key|Tab`
  (params (Key :type "Key Structure"))
  (bind _kernelhud (`/Game/PropHunt/Blueprints/Helpers/BP_Helpers.H_KernelHUD`))
  ;[1 1 1] Show Scoreboard
  (:`Pressed`
    (if (`|EnumEquality` (`/Game/PropHunt/Blueprints/Kernel/BP_Kernel_GS.GlobalState` (`/Game/PropHunt/Blueprints/Helpers/BP_Helpers.H_KernelGS`)) "NewEnumerator17")
      (`/Game/PropHunt/Blueprints/Kernel/BP_Kernel_HUD.F_ToggleGameChat` _kernelhud false)
      (`/Game/PropHunt/Blueprints/Kernel/BP_Kernel_HUD.F_ToggleScoreBoard` _kernelhud true)))
  (:`Released`
    (`/Game/PropHunt/Blueprints/Kernel/BP_Kernel_HUD.F_ToggleScoreBoard` _kernelhud false)))

(event `Key|Enter`
  (params (Key :type "Key Structure"))
  (bind _kernelhud (`/Game/PropHunt/Blueprints/Helpers/BP_Helpers.H_KernelHUD`))
  ;[0 0.6122 1] Open game chat
  (:`Pressed`
    (if (`|EnumEquality` (`/Game/PropHunt/Blueprints/Kernel/BP_Kernel_GS.GlobalState` (`/Game/PropHunt/Blueprints/Helpers/BP_Helpers.H_KernelGS`)) "NewEnumerator17")
      (`/Game/PropHunt/Blueprints/Kernel/BP_Kernel_HUD.F_ToggleGameChat` _kernelhud true)
      (`/Game/PropHunt/Blueprints/Widgets/Chat/BP_W_GameChat.E_OpenChat` (`/Game/PropHunt/Blueprints/Kernel/BP_Kernel_HUD.GameChat` _kernelhud)))))

(fn `IF_GetTeam`
  (returns (Team :type Integer))
  (bind _team (message `/Game/PropHunt/Blueprints/Interfaces/BP_I_TeamPlayer.IF_GetTeam` (`self.PlayerState`)))
  (return _team))

(fn `IF_SetTeam`
  (params (NewTeam :type Integer))
  (returns (Team :type Integer))
  (bind _team (message `/Game/PropHunt/Blueprints/Interfaces/BP_I_TeamPlayer.IF_SetTeam` (`self.PlayerState`) NewTeam))
  (return _team))

(fn `UserConstructionScript`)