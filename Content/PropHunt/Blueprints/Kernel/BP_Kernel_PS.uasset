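; PropHunt player state that holds each player's kills, deaths, score, team and dead flag, exposed through interface events and getters.
; On the server it binds to game state delegates to reset stats and award living team 1 players a round-end bonus.
; Score and death updates trigger client HUD events.
; In one specific game state, death also possesses a spawned observer pawn targeting the killer's character, with a fixed-location fallback.
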(event `self.ReceiveBeginPlay`
  ;[1 1 1] BEGIN PLAY
  (`/Engine/EditorBlueprintResources/ActorMacros.Switch Has Authority`
    (:`Authority`
      (add `/Game/PropHunt/Blueprints/Kernel/BP_Kernel_GS.D_LobbyState` (`/Game/PropHunt/Blueprints/Helpers/BP_Helpers.H_KernelGS`) (delegate `EA_ResetStats`))
      (add `/Game/PropHunt/Blueprints/Kernel/BP_Kernel_GS.D_RoundStart` (`/Game/PropHunt/Blueprints/Helpers/BP_Helpers.H_KernelGS`) (delegate `EA_ResetState`))
      (add `/Game/PropHunt/Blueprints/Kernel/BP_Kernel_GS.D_RoundFinish` (`/Game/PropHunt/Blueprints/Helpers/BP_Helpers.H_KernelGS`) (delegate `EA_UpdatePropScore`)))))

(event `EA_ResetState`
  ;[1 1 1] BEGIN PLAY
  (set `self.IsDead` false))

(event `EA_ResetStats`
  ;[1 1 1] BEGIN PLAY
  (`/Game/PropHunt/Blueprints/Interfaces/BP_I_PlayerStats.IE_ResetStats`))

(event `EA_UpdatePropScore`
  ;[1 1 1] BEGIN PLAY
  (if (and (== (`self.Team`) 1) (not (`self.IsDead`)))
    (`self.FS_UpdateScore` 300)))

(event `CL_OnDeath`
  (params (KillerId :type Integer))
  (bind _kernelhud (`/Game/PropHunt/Blueprints/Helpers/BP_Helpers.H_KernelHUD`))
  ;[1 1 1] On death
  (`/Engine/EditorBlueprintResources/StandardMacros.IsValid` _kernelhud
    (:`Is Valid`
      (`/Game/PropHunt/Blueprints/Kernel/BP_Kernel_HUD.F_RemoveAll` _kernelhud)
      (`/Game/PropHunt/Blueprints/Kernel/BP_Kernel_HUD.F_ToggleOserverHud` _kernelhud true KillerId))))

(event `/Game/PropHunt/Blueprints/Interfaces/BP_I_PlayerStats.IE_ResetStats`
  ;[1 1 1] Reset all stats
  (set `self.Kills` 0)
  (set `self.Deaths` 0)
  (set `self.MyScore` 0)
  (set `self.IsDead` false))

(event `/Game/PropHunt/Blueprints/Interfaces/BP_I_PlayerStats.IE_UpdateKills`
  ;[1 1 1] Update kills
  (`self.FS_IncrementKills`))

(event `/Game/PropHunt/Blueprints/Interfaces/BP_I_PlayerStats.IE_UpdateDeaths`
  (params (KillerId :type Integer))
  ;[1 1 1] Update deaths
  (`self.FS_IncrementDeaths`)
  (`self.CL_OnDeath` KillerId)
  (`self.FS_SpawnObserverPawn` KillerId))

(event `/Game/PropHunt/Blueprints/Interfaces/BP_I_PlayerStats.IE_UpdateScore`
  (params (AddScore :type Integer) (Message :type String))
  ;[1 1 1] Update score
  (`self.FS_UpdateScore` AddScore)
  (`self.CL_OnScoreUpdate` AddScore Message))

(event `CL_OnScoreUpdate`
  (params (Score :type Integer) (Message :type String))
  ;[1 1 1] Show notify and play sound on score update
  (`/Game/PropHunt/Blueprints/Kernel/BP_Kernel_HUD.F_ShowScoreNotify` (`/Game/PropHunt/Blueprints/Helpers/BP_Helpers.H_KernelHUD`) (`KismetStringLibrary.Conv_IntToString` Score) Message))

(fn `FS_IncrementDeaths`
  (returns (Deaths :type Integer))
  (bind _output_get (set `self.Deaths` (+ (`self.Deaths`) 1)))
  (return _output_get))

(fn `FS_IncrementKills`
  (returns (Kills :type Integer))
  (bind _output_get (set `self.Kills` (+ (`self.Kills`) 1)))
  (return _output_get))

(fn `FS_SpawnObserverPawn`
  (params (KillerId :type Integer))
  (locals (KillerCharacter :type "Character Object Reference"))
  (bind _foundps (`/Game/PropHunt/Blueprints/Helpers/BP_Helpers.H_GetPSFromPlayerArray` KillerId))
  (bind _asplayer_controller (cast `PlayerController` (`self.GetOwner`) :!pure true))
  (if (`|EnumEquality` (`/Game/PropHunt/Blueprints/Kernel/BP_Kernel_GS.GlobalState` (`/Game/PropHunt/Blueprints/Helpers/BP_Helpers.H_KernelGS`)) "NewEnumerator17")
    (`|ExecutionSequence`
      (:`then_0`
        (`/Engine/EditorBlueprintResources/StandardMacros.IsValid` _foundps
          (:`Is Valid`
            (bind _asplayer_controller_2 (cast `PlayerController` (`self.GetOwner` _foundps)))
            (bind _ascharacter (cast `Character` (`Controller.K2_GetPawn` _asplayer_controller_2)))
            (set `local.KillerCharacter` _ascharacter))))
      (:`then_1`
        (`/Engine/EditorBlueprintResources/StandardMacros.IsValid` (`local.KillerCharacter`)
          (:`Is Valid`
            (bind _camera (message `/Game/PropHunt/Blueprints/Interfaces/BP_I_BaseCharacter.IF_GetFollowCamera` (`Controller.K2_GetPawn` (cast `PlayerController` (`self.GetOwner`) :!pure true))))
            (bind _returnvalue (`|SpawnActorFromClass` (`self.ObserverClass`) (`KismetMathLibrary.MakeTransform` (`SceneComponent.K2_GetComponentLocation` _camera) (`SceneComponent.K2_GetComponentRotation` _camera)) "Undefined" "OverrideRootScale" _asplayer_controller (`local.KillerCharacter`) null))
            (`Controller.Possess` _asplayer_controller _returnvalue))
          (:`Is Not Valid`
            (bind _returnvalue_2 (`|SpawnActorFromClass` (`self.ObserverClass`) (`KismetMathLibrary.MakeTransform` (0.0 0.0 1000.0)) "Undefined" "OverrideRootScale" null null null))
            (`Controller.Possess` (cast `PlayerController` (`self.GetOwner`) :!pure true) _returnvalue_2)))))))

(fn `FS_UpdateScore`
  (params (AddScore :type Integer))
  (returns (Score :type Integer))
  (bind _output_get (set `self.MyScore` (+ AddScore (`self.MyScore`))))
  (return _output_get))

(fn `IF_GetDeaths`
  (returns (deaths :type Integer))
  (return (`self.Deaths`)))

(fn `IF_GetKills`
  (returns (kills :type Integer))
  (return (`self.Kills`)))

(fn `IF_GetScore`
  (returns (score :type Integer))
  (return (`self.MyScore`)))

(fn `IF_GetTeam`
  (returns (Team :type Integer))
  (return (`self.Team`)))

(fn `IF_SetTeam`
  (params (NewTeam :type Integer))
  (returns (Team :type Integer))
  (bind _output_get (set `self.Team` NewTeam))
  (return _output_get))

(fn `UserConstructionScript`)