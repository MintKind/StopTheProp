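; Main menu HUD for PropHunt that owns and switches the front-end widgets, showing the background, Home menu and mouse cursor on BeginPlay.
; Each screen has a toggle function that lazily creates and caches its widget, re-adding it only when not visible.
; Connect-loading and network-error overlays are created at a higher Z-order, with the error fed the last error message.
; A reset function removes and clears the five menu screens, leaving the background.
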(event `self.ReceiveBeginPlay`
  (`self.F_ShowBG`)
  (`self.F_ToggleHomeMenu` true)
  (set `PlayerController.bShowMouseCursor` true (`self.PlayerOwner`)))

(fn `F ToggleNetworkError`
  (params (Show :type Boolean))
  (bind _networkerror (`self.NetworkError`))
  (if Show
    (`self.NetworkError`
      (:`then`
        (`/Game/PropHunt/Blueprints/Helpers/BP_MacroHelpers.MH_IsWidgetVisible` _networkerror
          (:`false`
            (`UserWidget.AddToViewport` _networkerror 0))))
      (:`else`
        (bind _returnvalue (`|CreateWidget` "/Game/PropHunt/Blueprints/Widgets/MainMenu/BP_W_NetworkError.BP_W_NetworkError_C" (`self.PlayerOwner`) (`KismetTextLibrary.Conv_TextToString` (`SourceControlHelpers.LastErrorMsg`))))
        (bind _output_get (set `self.NetworkError` _returnvalue))
        (`UserWidget.AddToViewport` _output_get 22)))
    (else
      (bind _networkerror_2 (`self.NetworkError`)
        (:`then`
          (`Widget.RemoveFromParent` _networkerror_2))
        (:`else`)))))

(fn `F_RemoveAllExceptBg`
  (`|ExecutionSequence`
    (:`then_0`
      (bind _faq (`self.Faq`)
        (:`then`
          (`Widget.RemoveFromParent` _faq)
          (set `self.Faq` null))
        (:`else`)))
    (:`then_1`
      (bind _home (`self.Home`)
        (:`then`
          (`Widget.RemoveFromParent` _home)
          (set `self.Home` null))
        (:`else`)))
    (:`then_2`
      (bind _hostgame (`self.HostGame`)
        (:`then`
          (`Widget.RemoveFromParent` _hostgame)
          (set `self.HostGame` null))
        (:`else`)))
    (:`then_3`
      (bind _serverbrowser (`self.ServerBrowser`)
        (:`then`
          (`Widget.RemoveFromParent` _serverbrowser)
          (set `self.ServerBrowser` null))
        (:`else`)))
    (:`then_4`
      (bind _settings (`self.Settings`)
        (:`then`
          (`Widget.RemoveFromParent` _settings)
          (set `self.Settings` null))
        (:`else`)))))

(fn `F_ShowBG`
  (bind _returnvalue (`|CreateWidget` "/Game/PropHunt/Blueprints/Widgets/MainMenu/BP_W_BG.BP_W_BG_C" (`self.PlayerOwner`)))
  (`UserWidget.AddToViewport` _returnvalue 0))

(fn `F_ToggleFaqMenu`
  (params (Show :type Boolean))
  (bind _faq (`self.Faq`))
  (if Show
    (`self.Faq`
      (:`then`
        (`/Game/PropHunt/Blueprints/Helpers/BP_MacroHelpers.MH_IsWidgetVisible` _faq
          (:`false`
            (`UserWidget.AddToViewport` _faq 0))))
      (:`else`
        (bind _returnvalue (`|CreateWidget` "/Game/PropHunt/Blueprints/Widgets/MainMenu/BP_W_FAQ.BP_W_FAQ_C" (`self.PlayerOwner`)))
        (bind _output_get (set `self.Faq` _returnvalue))
        (`UserWidget.AddToViewport` _output_get 0)))
    (else
      (bind _faq_2 (`self.Faq`)
        (:`then`
          (`Widget.RemoveFromParent` _faq_2))
        (:`else`)))))

(fn `F_ToggleHomeMenu`
  (params (Show :type Boolean))
  (bind _home (`self.Home`))
  (if Show
    (`self.Home`
      (:`then`
        (`/Game/PropHunt/Blueprints/Helpers/BP_MacroHelpers.MH_IsWidgetVisible` _home
          (:`false`
            (`UserWidget.AddToViewport` _home 0))))
      (:`else`
        (bind _returnvalue (`|CreateWidget` "/Game/PropHunt/Blueprints/Widgets/MainMenu/BP_W_Home.BP_W_Home_C" (`self.PlayerOwner`)))
        (bind _output_get (set `self.Home` _returnvalue))
        (`UserWidget.AddToViewport` _output_get 0)))
    (else
      (bind _home_2 (`self.Home`)
        (:`then`
          (`Widget.RemoveFromParent` _home_2))
        (:`else`)))))

(fn `F_ToggleHostGameMenu`
  (params (Show :type Boolean))
  (bind _hostgame (`self.HostGame`))
  (if Show
    (`self.HostGame`
      (:`then`
        (`/Game/PropHunt/Blueprints/Helpers/BP_MacroHelpers.MH_IsWidgetVisible` _hostgame
          (:`false`
            (`UserWidget.AddToViewport` _hostgame 0))))
      (:`else`
        (bind _returnvalue (`|CreateWidget` "/Game/PropHunt/Blueprints/Widgets/MainMenu/BP_W_HostGame.BP_W_HostGame_C" (`self.PlayerOwner`)))
        (bind _output_get (set `self.HostGame` _returnvalue))
        (`UserWidget.AddToViewport` _output_get 0)))
    (else
      (bind _hostgame_2 (`self.HostGame`)
        (:`then`
          (`Widget.RemoveFromParent` _hostgame_2))
        (:`else`)))))

(fn `F_ToggleServerBrowserMenu`
  (params (Show :type Boolean))
  (bind _serverbrowser (`self.ServerBrowser`))
  (if Show
    (`self.ServerBrowser`
      (:`then`
        (`/Game/PropHunt/Blueprints/Helpers/BP_MacroHelpers.MH_IsWidgetVisible` _serverbrowser
          (:`false`
            (`UserWidget.AddToViewport` _serverbrowser 0))))
      (:`else`
        (bind _returnvalue (`|CreateWidget` "/Game/PropHunt/Blueprints/Widgets/MainMenu/BP_W_ServerBrowser.BP_W_ServerBrowser_C" (`self.PlayerOwner`)))
        (bind _output_get (set `self.ServerBrowser` _returnvalue))
        (`UserWidget.AddToViewport` _output_get 0)))
    (else
      (bind _serverbrowser_2 (`self.ServerBrowser`)
        (:`then`
          (`Widget.RemoveFromParent` _serverbrowser_2))
        (:`else`)))))

(fn `F_ToggleSessionConnectLoading`
  (params (Show :type Boolean))
  (bind _sessionconnectloading (`self.SessionConnectLoading`))
  (if Show
    (`self.SessionConnectLoading`
      (:`then`
        (`/Game/PropHunt/Blueprints/Helpers/BP_MacroHelpers.MH_IsWidgetVisible` _sessionconnectloading
          (:`false`
            (`UserWidget.AddToViewport` _sessionconnectloading 0))))
      (:`else`
        (bind _returnvalue (`|CreateWidget` "/Game/PropHunt/Blueprints/Widgets/MainMenu/BP_W_ConnectLoading.BP_W_ConnectLoading_C" (`self.PlayerOwner`)))
        (bind _output_get (set `self.SessionConnectLoading` _returnvalue))
        (`UserWidget.AddToViewport` _output_get 22)))
    (else
      (bind _sessionconnectloading_2 (`self.SessionConnectLoading`)
        (:`then`
          (`Widget.RemoveFromParent` _sessionconnectloading_2))
        (:`else`)))))

(fn `F_ToggleSettingsMenu`
  (params (Show :type Boolean))
  (bind _settings (`self.Settings`))
  (if Show
    (`self.Settings`
      (:`then`
        (`/Game/PropHunt/Blueprints/Helpers/BP_MacroHelpers.MH_IsWidgetVisible` _settings
          (:`false`
            (`UserWidget.AddToViewport` _settings 0))))
      (:`else`
        (bind _returnvalue (`|CreateWidget` "/Game/PropHunt/Blueprints/Widgets/MainMenu/BP_W_Settings.BP_W_Settings_C" (`self.PlayerOwner`)))
        (bind _output_get (set `self.Settings` _returnvalue))
        (`UserWidget.AddToViewport` _output_get 0)))
    (else
      (bind _settings_2 (`self.Settings`)
        (:`then`
          (`Widget.RemoveFromParent` _settings_2))
        (:`else`)))))

(fn `UserConstructionScript`)