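; Base projectile actor for PropHunt weapons that travels briefly and shows impact effects.
; On spawn, its collision ignores the owner and instigator while moving, and a short lifespan is set.
; On hit, it spawns the assault rifle impact particle unless it struck a Character, then destroys itself.
; The Blueprint applies no damage in its graph.
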(event `self.ReceiveBeginPlay`
  (`PrimitiveComponent.IgnoreActorWhenMoving` (`self.Collision`) (`self.GetOwner`) true)
  (`PrimitiveComponent.IgnoreActorWhenMoving` (`self.Collision`) (`self.GetInstigator`) true)
  (`self.SetLifeSpan` 1.0))

(event `self.ReceiveHit`
  (params (MyComp :type "PrimitiveComponent Object Reference") (Other :type "Actor Object Reference") (OtherComp :type "PrimitiveComponent Object Reference") (bSelfMoved :type Boolean) (HitLocation :type "Vector Structure") (HitNormal :type "Vector Structure") (NormalImpulse :type "Vector Structure") (Hit :type "HitResult Structure (by ref)"))
  (cast `Character` Other
    (:`then`
      _)
    (:`CastFailed`
      (`GameplayStatics.SpawnEmitterAtLocation` "/Game/PropHunt/Content/Effects/PS_AssaultRifle_HIT.PS_AssaultRifle_HIT" HitLocation)))
  (`self.K2_DestroyActor`))

(fn `UserConstructionScript`)