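; Base firearm actor for the PropHunt hunters, handling equip, holster, drop, aim zoom, single or auto fire, and reload.
; Firing splits into predicted local effects and cosmetic projectiles, plus server-timed camera line traces that apply damage and multicast effects to other clients.
; Shooting a non-player prop damages the shooting hunter to discourage spraying every prop.
; Ammo is tracked on the server, and reload completes after the montage length unless aborted.
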(event `self.ReceiveBeginPlay`
  ;[1 0 0] begin play. set ammo
  (`/Engine/EditorBlueprintResources/ActorMacros.Switch Has Authority`
    (:`Authority`
      (set `self.Ammo` (`self.MaxAmmo`))
      (set `self.BulletsInMagazin` (`self.MaxBulletsInMagazine`)))))

(event `MC_Equip`
  (params (Character :type "Character Object Reference"))
  ;[1 1 1] Play equip montage on all clients
  (`/Engine/EditorBlueprintResources/StandardMacros.IsValid` Character
    (:`Is Valid`
      (`Character.PlayAnimMontage` Character (`self.CharEquipAnimation`) 1.0 "None"))))

(event `EA_Equip`
  ;[1 0 0] EQUIP weapon
  (`|ExecutionSequence`
    (:`then_0`
      (`PrimitiveComponent.SetCollisionResponseToChannel` (`self.FocusCollision`) "ECC_Visibility" "ECR_Ignore")
      (set `self.WeaponLocation` "NewEnumerator1")
      (set `self.IsEquiping` true)
      (`KismetSystemLibrary.Delay` (- (`AnimSequenceBase.SequenceLength` (`self.CharEquipAnimation`)) 0.2))
      (set `self.IsEquiping` false))
    (:`then_1`
      (`self.MC_Equip` (`self.OwnerCharacter`))
      (`self.K2_AttachToComponent` (`Character.Mesh` (`self.OwnerCharacter`)) "rhand" "SnapToTarget" "SnapToTarget" "SnapToTarget" false))))

(event `self.IE_ShotReleased`
  ;[0 1 0.05132] Shoot released
  (`self.F_StopLocalAutoFire`)
  (`self.SRV_ShootReleased`))

(event `SRV_ShootPressed`
  ;[1 1 1] Single shoot or autofire on server
  (if (`self.F_CanShoot`)
    (switch `/Game/PropHunt/Blueprints/Weapons/E_ShotingMode` (`self.ShotingMode`)
      (:`NewEnumerator1`
        (`self.FS_StartServerAutoFireTimer`))
      (:`NewEnumerator0`
        (`self.EA_Shoot`)))
    (else
      (`self.FS_StopServerAutoFire`))))

(event `SRV_ShootReleased`
  ;[0 1 0.05132] Shoot released
  (`self.FS_StopServerAutoFire`))

(event `self.IE_ShotPressed`
  ;[0 0.1378 1] Shoot pressed.
  ; Start local autofire timer (show shot effects)
  (if (`self.F_CanShoot`)
    (switch `/Game/PropHunt/Blueprints/Weapons/E_ShotingMode` (`self.ShotingMode`)
      (:`NewEnumerator1`
        (`self.F_StartLocalAutoFireTimer`)
        (`self.SRV_ShootPressed`))
      (:`NewEnumerator0`
        (`self.F_LocalSingleShootEffects`)
        (`self.SRV_ShootPressed`)))
    (else
      (`self.F_StopLocalAutoFire`))))

(event `EA_Holster`
  ;[1 0.5771 0] Holster weapon
  (`self.K2_AttachToComponent` (`Character.Mesh` (`self.OwnerCharacter`)) (`self.F_GetHolsterSocket`) "SnapToTarget" "SnapToTarget" "SnapToTarget" false)
  (set `self.WeaponLocation` "NewEnumerator2"))

(event `self.IE_Aim`
  (params (Aim :type Boolean))
  ;[0 1 0.6366] AIM
  (if Aim
    (bind (_direction _zoom) (`Timeline|Timeline_0` :!label _label)
      (:`Update`
        (bind _camera (message `/Game/PropHunt/Blueprints/Interfaces/BP_I_BaseCharacter.IF_GetFollowCamera` (`self.OwnerCharacter`)))
        (`CameraComponent.SetFieldOfView` _camera (`KismetMathLibrary.Lerp` 90.0 (`self.AimFOV`) _zoom))))
    (else
      (goto _label :!via `Reverse`))))

(event `self.IE_Reload`
  (bind _charreloadanimation (`self.CharReloadAnimation`))
  ;[0.8684 0.02316 1] RELOAD - only on server
  (`self.FS_StopServerAutoFire`)
  (`/Engine/EditorBlueprintResources/StandardMacros.IsValid` _charreloadanimation
    (:`Is Valid`
      (`KismetSystemLibrary.Delay` (- (`AnimSequenceBase.SequenceLength` _charreloadanimation) 0.2))
      (bind _asbp_hunter_character (cast `/Game/PropHunt/Blueprints/Characters/BP_HunterCharacter` (`self.OwnerCharacter`))
        (:`then`
          (bind _bp_weaponsmanager (`/Game/PropHunt/Blueprints/Characters/BP_HunterCharacter.BP_WeaponsManager` _asbp_hunter_character))
          (`/Engine/EditorBlueprintResources/StandardMacros.IsValid` _bp_weaponsmanager
            (:`Is Valid`
              (if (not (`/Game/PropHunt/Blueprints/Characters/BP_WeaponsManager.WasReloadingAborted` _bp_weaponsmanager))
                (`self.FS_Reload`)))
            (:`Is Not Valid`
              (`self.FS_Reload` :!label _label_2))))
        (:`CastFailed`
          (goto _label_2))))
    (:`Is Not Valid`
      (`self.FS_Reload`))))

(event `EA_Drop`
  ;[0 0.9966 1] Drop Weapon
  (`self.K2_SetActorLocation` (+ (`self.K2_GetActorLocation` (`self.OwnerCharacter`)) (`KismetMathLibrary.MakeVector` (`KismetMathLibrary.RandomFloatInRange` 40.0 70.0) (`KismetMathLibrary.RandomFloatInRange` 40.0 70.0) -90.0)))
  (`self.K2_SetActorRotation` (struct))
  (`self.K2_DetachFromActor` "KeepWorld" "KeepWorld" "KeepWorld")
  (`PrimitiveComponent.SetCollisionResponseToChannel` (`self.FocusCollision`) "ECC_Visibility" "ECR_Block")
  (set `self.OwnerCharacter` null)
  (set `self.WeaponLocation` "NewEnumerator3")
  (`self.SetOwner` null))

(event `EA_Shoot`
  (bind (_tracestart _traceend) (`self.F_GetBulletTrace`))
  ;[1 1 1] Shot
  (`/Engine/EditorBlueprintResources/ActorMacros.Switch Has Authority`
    (:`Authority`
      (if (`self.F_CanShoot`)
        (`|ExecutionSequence`
          (:`then_0`
            (`self.MC_ShootEffects` _tracestart _traceend)
            (bind (_outhit _returnvalue) (`KismetSystemLibrary.LineTraceSingle` _tracestart _traceend "TraceTypeQuery3"))
            (if _returnvalue
              (bind _damag (`self.IF_GetDamage`))
              (bind (_bblockinghit _binitialoverlap _time _distance _location _impactpoint _normal _impactnormal _physmat _hitactor) (`GameplayStatics.BreakHitResult` _outhit))
              (cast `Character` _hitactor
                (:`then`
                  (`GameplayStatics.ApplyPointDamage` _hitactor _damag _impactpoint _outhit (`Pawn.GetController` (`self.OwnerCharacter`)) self)
                  (`self.MC_BloodHitEffect` _location))
                (:`CastFailed`
                  ;;[1 0 0.1038] If hunter shots in prop which is not prop character, apply damage to hunter
                  ;; We do it to avoid situation when hunter shots in every prop without any limitations
                  (cast `/Game/PropHunt/Blueprints/Props/BP_BaseProp` _hitactor)
                  (bind _asbp_hunter_character (cast `/Game/PropHunt/Blueprints/Characters/BP_HunterCharacter` (`self.OwnerCharacter`)))
                  (`/Game/PropHunt/Blueprints/Characters/BP_HunterCharacter.SRV_ApplyDamage` _asbp_hunter_character)))))
          (:`then_1`
            (bind _isempty (`self.FS_DecreaseAmmo`))
            (if _isempty
              (message `/Game/PropHunt/Blueprints/Interfaces/BP_I_ArmedCharacter.IE_Reload` (`self.OwnerCharacter`)))))
        (else
          (`self.FS_StopServerAutoFire`))))))

(event `MC_ShootEffects`
  (params (Start :type "Vector Structure") (End :type "Vector Structure"))
  (bind _ownercharacter (`self.OwnerCharacter`))
  ;[1 0.9962 0] Multicast shot effects
  (`/Engine/EditorBlueprintResources/StandardMacros.IsValid` _ownercharacter
    (:`Is Valid`
      (if (not (`Pawn.IsLocallyControlled` _ownercharacter))
        (`self.F_LocalSingleShootEffects`)
        (`self.F Spawn Projectile` Start End)))))

(event `MC_BloodHitEffect`
  (params (Location :type "Vector Structure"))
  ;[1 0.9962 0] Multicast blood effect
  (`GameplayStatics.SpawnEmitterAtLocation` "/Game/PropHunt/Content/Effects/BloodHitEffect/PS_body_bullet_impact.PS_body_bullet_impact" Location))

(fn `F Spawn Projectile`
  (params (Start :type "Vector Structure") (End :type "Vector Structure"))
  (bind _outhit (`KismetSystemLibrary.LineTraceSingle` Start End "TraceTypeQuery3" false (`|MakeArray` (`self.OwnerCharacter`) :!type "Actor Object Reference")))
  (bind (_bblockinghit _binitialoverlap _time _distance _location _impactpoint _normal _impactnormal _physmat _hitactor _hitcomponent _hitbonename _hititem _faceindex _tracestart _traceend) (`GameplayStatics.BreakHitResult` _outhit))
  (`|SpawnActorFromClass` (`self.ProjectileClass`) (`self.F_GetProjectileSpawnLocation` _bblockinghit _location _traceend) "AlwaysSpawn" "OverrideRootScale" self (`self.OwnerCharacter`)))

(fn `F_CanShoot`
  (returns (Shoot :type Boolean))
  (return (and (> (`self.BulletsInMagazin`) 0) (not (`self.IsEquiping`)))))

(fn `F_GetBulletTrace`
  (returns (TraceStart :type "Vector Structure") (TraceEnd :type "Vector Structure"))
  (bind _camera (message `/Game/PropHunt/Blueprints/Interfaces/BP_I_BaseCharacter.IF_GetFollowCamera` (`self.OwnerCharacter`)))
  (bind _returnvalue (`SceneComponent.K2_GetComponentLocation` _camera))
  (bind _returnvalue_2 (`SceneComponent.GetForwardVector` _camera))
  (return (+ _returnvalue (* _returnvalue_2 300.0)) (+ _returnvalue (* _returnvalue_2 100000.0))))

(fn `F_GetHolsterSocket`
  (returns (socket :type Name))
  (switch `/Game/PropHunt/Blueprints/Weapons/E_WeaponType` (`self.WeaponType`)
    (:`NewEnumerator0`
      (return "pw"))
    (:`NewEnumerator1`
      (return "sw"))))

(fn `F_GetProjectileSpawnLocation`
  (params (WasHit :type Boolean) (HitLocation :type "Vector Structure") (TraceEnd :type "Vector Structure"))
  (returns (SpawnLocation :type "Transform Structure"))
  (locals (HitLocation_L :type "Vector Structure") (Rotation_L :type "Rotator Structure") (MuzzleSocketLocation_L :type "Vector Structure") (TraceEnd_L :type "Vector Structure") (WasHit_L :type Boolean))
  (bind _returnvalue (`SceneComponent.GetSocketLocation` (`self.WeaponSM`) (`self.MuzzleSocket`)))
  (set `local.WasHit_L` WasHit)
  (set `local.HitLocation_L` HitLocation)
  (set `local.TraceEnd_L` TraceEnd)
  (`|ExecutionSequence`
    (:`then_0`
      (set `local.MuzzleSocketLocation_L` _returnvalue)
      (if (`local.WasHit_L`)
        (set `local.Rotation_L` (`KismetMathLibrary.FindLookAtRotation` _returnvalue (`local.HitLocation_L`)))
        (else
          (set `local.Rotation_L` (`KismetMathLibrary.FindLookAtRotation` (`local.MuzzleSocketLocation_L`) (`local.TraceEnd_L`))))))
    (:`then_1`
      (return (`KismetMathLibrary.MakeTransform` (`local.MuzzleSocketLocation_L`) (`local.Rotation_L`))))))

(fn `F_LocalSingleShootEffects`
  (bind (_tracestart _traceend) (`self.F_GetBulletTrace`))
  (bind _kernelhud (`/Game/PropHunt/Blueprints/Helpers/BP_Helpers.H_KernelHUD`))
  (bind (_tracestart_2 _traceend_2) (`self.F_GetBulletTrace`))
  (if (`self.F_CanShoot`)
    (`|ExecutionSequence`
      (:`then_0`
        (if (`Pawn.IsLocallyControlled` (`self.OwnerCharacter`))
          (`self.F Spawn Projectile` _tracestart _traceend)))
      (:`then_1`
        (`GameplayStatics.PlayWorldCameraShake` "/Game/PropHunt/Blueprints/Weapons/BP_CameraRecoilShake.BP_CameraRecoilShake_C" (`self.K2_GetActorLocation`) 0.0 500.0 1.0 true)
        (`GameplayStatics.PlaySoundAtLocation` "/Game/PropHunt/Content/Sounds/S_Rifle_Shot_Cue.S_Rifle_Shot_Cue" (`SceneComponent.K2_GetComponentLocation` (`self.WeaponSM`)) (struct) 1.0 1.0 0.0 null null null)
        (`GameplayStatics.SpawnEmitterAttached` "/Game/PropHunt/Content/Effects/PS_AssaultRifle_MF.PS_AssaultRifle_MF" (`self.WeaponSM`) (`self.MuzzleSocket`) (0.0 0.0 0.0) (struct) (1.0 1.0 1.0) "SnapToTargetIncludingScale")
        (bind (_outhit _returnvalue) (`KismetSystemLibrary.LineTraceSingle` _tracestart_2 _traceend_2 "TraceTypeQuery3"))
        (if _returnvalue
          (cast `Character` (`.HitActor` (`GameplayStatics.BreakHitResult` _outhit)))
          (if (== (`GameplayStatics.GetPlayerCharacter` 0) (`self.OwnerCharacter`))
            (`/Engine/EditorBlueprintResources/StandardMacros.IsValid` _kernelhud
              (:`Is Valid`
                (`/Game/PropHunt/Blueprints/Kernel/BP_Kernel_HUD.E_ShowHitIndicator` _kernelhud)))))))
    (else
      (`self.F_StopLocalAutoFire`))))

(fn `F_StartLocalAutoFireTimer`
  ;[1 1 1] First delay compensation
  (`self.F_LocalSingleShootEffects`)
  (bind _returnvalue (`KismetSystemLibrary.K2_SetTimer` null "F_LocalSingleShootEffects" (/ 1.0 (`KismetMathLibrary.Conv_IntToDouble` (`self.ShotsPerSec`))) true))
  (set `self.LocalAutoFireTimer` _returnvalue))

(fn `F_StopLocalAutoFire`
  (`KismetSystemLibrary.K2_ClearAndInvalidateTimerHandle` (`self.LocalAutoFireTimer`)))

(fn `FS_DecreaseAmmo`
  (returns (IsEmpty :type Boolean))
  (bind _output_get (set `self.BulletsInMagazin` (- (`self.BulletsInMagazin`) 1)))
  (return (<= _output_get 0)))

(fn `FS_Reload`
  (locals (RemainingAmmo :type Integer) (RemainingBulletsInMag :type Integer) (NeedAmmo :type Integer) (MaxBulletsInMag :type Integer))
  (set `local.RemainingAmmo` (`self.Ammo`))
  (set `local.RemainingBulletsInMag` (`self.BulletsInMagazin`))
  (set `local.MaxBulletsInMag` (`self.MaxBulletsInMagazine`))
  (if (== (`self.BulletsInMagazin`) 0)
    (if (>= (`self.Ammo`) (`local.MaxBulletsInMag`))
      (set `self.Ammo` (- (`self.Ammo`) (`local.MaxBulletsInMag`)))
      (set `self.BulletsInMagazin` (`local.MaxBulletsInMag`))
      (else
        (set `self.BulletsInMagazin` (`local.RemainingAmmo`))
        (set `self.Ammo` 0)))
    (else
      (set `local.NeedAmmo` (- (`local.MaxBulletsInMag`) (`local.RemainingBulletsInMag`)))
      (if (>= (`self.Ammo`) (`local.NeedAmmo`))
        (set `self.Ammo` (- (`self.Ammo`) (`local.NeedAmmo`)))
        (set `self.BulletsInMagazin` (`local.MaxBulletsInMag`))
        (else
          (set `self.BulletsInMagazin` (`local.RemainingAmmo`))
          (set `self.Ammo` 0))))))

(fn `FS_SetOwner`
  (params (NewOwner :type "Actor Object Reference"))
  (`self.SetOwner` NewOwner)
  (bind _ascharacter (cast `Character` NewOwner))
  (set `self.OwnerCharacter` _ascharacter)
  (`PrimitiveComponent.SetCollisionResponseToChannel` (`self.FocusCollision`) "ECC_Visibility" "ECR_Ignore"))

(fn `FS_StartServerAutoFireTimer`
  ;[1 1 1] First delay compensation
  (`self.EA_Shoot`)
  (bind _returnvalue (`KismetSystemLibrary.K2_SetTimer` null "EA_Shoot" (/ 1.0 (`KismetMathLibrary.Conv_IntToDouble` (`self.ShotsPerSec`))) true))
  (set `self.ServerAutoFireTimer` _returnvalue))

(fn `FS_StopServerAutoFire`
  (`KismetSystemLibrary.K2_ClearAndInvalidateTimerHandle` (`self.ServerAutoFireTimer`)))

(fn `IF_CanFocus`
  (returns (CanFocus :type Boolean))
  (return (`|EnumEquality` (`self.WeaponLocation`) "NewEnumerator3")))

(fn `IF_CanPickUp`
  (returns (CanPickUp :type Boolean))
  (return false))

(fn `IF_CanReload`
  (returns (CanReload :type Boolean))
  (return (and (!= (`self.BulletsInMagazin`) (`self.MaxBulletsInMagazine`)) (> (`self.Ammo`) 0))))

(fn `IF_GetDamage`
  (returns (Damag :type "Float (double-precision)"))
  (return (`self.Damage`)))

(fn `IF_GetWeaponLocation`
  (returns (Location :type "/Game/PropHunt/Blueprints/Weapons/E_WeaponLocation Enum"))
  (return (`self.WeaponLocation`)))

(fn `IF_GetWeaponType`
  (returns (Type :type "/Game/PropHunt/Blueprints/Weapons/E_WeaponType Enum"))
  (return (`self.WeaponType`)))

(fn `UserConstructionScript`)